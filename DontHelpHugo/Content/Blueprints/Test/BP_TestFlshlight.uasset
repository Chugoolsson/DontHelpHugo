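; Flashlight equipment that reveals hidden messages and fires battery-powered bullets.
; RevealCollision overlaps show or hide messages through a CBP_Reveal component, falling back to the BI_Reveal interface.
; Self-rescheduling named timers drain and recharge the battery, updating a widget and toggling light and collision when empty, charging or full.
; Equipment abilities fire a bullet at a battery cost or start and stop charging, while pickup and drop toggle the UI.
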(event OnComponentBeginOverlap(RevealCollision)
  (params (OverlappedComponent :type Primitive%20Component%20Object%20Reference) (OtherActor :type Actor%20Object%20Reference) (OtherComp :type Primitive%20Component%20Object%20Reference) (OtherBodyIndex :type Integer) (bFromSweep :type Boolean) (SweepResult :type Hit%20Result%20Structure%20%28by%20ref%29))
  (bind _returnvalue (Actor|GetComponentbyClass OtherActor "/Game/Blueprints/LvL_TheFlashight/Actor_Components/CBP_Reveal.CBP_Reveal_C"))
  (Utilities|IsValid _returnvalue
    (:Is%20Valid
      (Class|BIReveal|Reveal(Message) _returnvalue))
    (:Is%20Not%20Valid
      (if (Utilities|DoesObjectImplementInterface OtherActor "/Game/Blueprints/LvL_TheFlashight/Interfaces/BI_Reveal.BI_Reveal_C")
        (Class|BIReveal|Reveal(Message) OtherActor)))))

(event OnComponentEndOverlap(RevealCollision)
  (params (OverlappedComponent :type Primitive%20Component%20Object%20Reference) (OtherActor :type Actor%20Object%20Reference) (OtherComp :type Primitive%20Component%20Object%20Reference) (OtherBodyIndex :type Integer))
  (bind _returnvalue (Actor|GetComponentbyClass OtherActor "/Game/Blueprints/LvL_TheFlashight/Actor_Components/CBP_Reveal.CBP_Reveal_C"))
  (Utilities|IsValid _returnvalue
    (:Is%20Valid
      (Class|BIReveal|Hide(Message) _returnvalue))
    (:Is%20Not%20Valid
      (if (Utilities|DoesObjectImplementInterface OtherActor "/Game/Blueprints/LvL_TheFlashight/Interfaces/BI_Reveal.BI_Reveal_C")
        (Class|BIReveal|Hide(Message) OtherActor)))))

(event Custom|Charging%20Battery
  (Utilities|Time|PauseTimerbyHandle (Variables|Default|GetTimeHandleLoosingBattery))
  (Variables|Default|SetCurrentBattery (Math|Float|Clamp(Float) (+ (Variables|Default|GetCurrentBattery) (Variables|Default|GetAddBattery)) 0.0 (Variables|Default|GetMaxBattery)))
  (Class|BIUpdateUI|UpdateUI(Message) (Variables|Default|GetFlashlightUI) (/ (Variables|Default|GetCurrentBattery) (Variables|Default|GetMaxBattery)))
  (if (== (Variables|Default|GetCurrentBattery) (Variables|Default|GetMaxBattery))
    (Utilities|Time|PauseTimerbyHandle (Variables|Default|GetTimeHandlerChargingBattery))
    (Rendering|SetVisibility (Variables|Default|GetSpotLight) true false)
    (Rendering|SetVisibility (Variables|Default|GetRevealCollision) true false)
    (CallFunction|TurnonLightCollision)
    (Utilities|Time|SetTimerbyFunctionName 0 "Loosing Battery" (Variables|Default|GetReduceBattery))
    (Variables|Default|SetisCharging false)
    (else
      (bind _returnvalue (Utilities|Time|SetTimerbyFunctionName 0 "Charging Battery" (Variables|Default|GetChargeTime)))
      (Variables|Default|SetTimeHandlerChargingBattery _returnvalue))))

(event Custom|Loosing%20Battery
  (Variables|Default|SetCurrentBattery (Math|Float|Clamp(Float) (- (Variables|Default|GetCurrentBattery) (Variables|Default|GetReduceBattery)) 0.0 (Variables|Default|GetMaxBattery)))
  (Class|BIUpdateUI|UpdateUI(Message) (Variables|Default|GetFlashlightUI) (/ (Variables|Default|GetCurrentBattery) (Variables|Default|GetMaxBattery)))
  (if (Variables|Default|GetpickedUp)
    (if (== (Variables|Default|GetCurrentBattery) 0.0)
      (Rendering|SetVisibility (Variables|Default|GetSpotLight) false false)
      (Rendering|SetVisibility (Variables|Default|GetRevealCollision) false false)
      (CallFunction|TurnOffLightCollision)
      (else
        (bind _returnvalue (Utilities|Time|SetTimerbyFunctionName 0 "Loosing Battery" (Variables|Default|GetReduceBattery)))
        (Variables|Default|SetTimeHandleLoosingBattery _returnvalue)))))

(event Event1stEquipmentAbility
  (if (not (Variables|Default|GetisCharging))
    (if (>= (Variables|Default|GetCurrentBattery) 2e+01)
      (CallFunction|ShootBullet)
      (Variables|Default|SetCurrentBattery (- (Variables|Default|GetCurrentBattery) 2e+01))
      (Class|BIUpdateUI|UpdateUI(Message) (Variables|Default|GetFlashlightUI) (/ (Variables|Default|GetCurrentBattery) (Variables|Default|GetMaxBattery)))
      (if (== (Variables|Default|GetCurrentBattery) 0.0)
        (Rendering|SetVisibility (Variables|Default|GetSpotLight) false false)
        (Rendering|SetVisibility (Variables|Default|GetRevealCollision) false false)
        (Collision|SetCollisionEnabled (Variables|Default|GetRevealCollision) "NoCollision")))))

(event Event3rdEquipmentAbility
  (Variables|Default|SetisCharging true)
  (bind _returnvalue (Utilities|Time|SetTimerbyFunctionName 0 "Charging Battery" (Variables|Default|GetChargeTime)))
  (Variables|Default|SetTimeHandlerChargingBattery _returnvalue)
  (Rendering|SetVisibility (Variables|Default|GetSpotLight) false false)
  (Rendering|SetVisibility (Variables|Default|GetRevealCollision) false false)
  (CallFunction|TurnOffLightCollision))

(event EventBeginPlay
  (Variables|Default|SetCurrentAmmo (Variables|Default|GetMaxAmmo))
  (Variables|Default|SetCurrentBattery (Variables|Default|GetMaxBattery))
  (CallFunction|SetUpWidgets))

(event EventPickedUp
  (Widget|SetVisibility (Variables|Default|GetFlashlightUI) "Visible")
  (bind _returnvalue (Utilities|Time|SetTimerbyFunctionName 0 "Loosing Battery" (Variables|Default|GetReduceBattery)))
  (Variables|Default|SetTimeHandlerChargingBattery _returnvalue))

(event EventTick
  (params (DeltaSeconds :type Float%20%28single-precision%29)))

(event EventDropped
  (CallFunction|TurnonLightCollision)
  (Rendering|SetVisibility (Variables|Default|GetSpotLight) true false)
  (Rendering|SetVisibility (Variables|Default|GetRevealCollision) true false)
  (Widget|SetVisibility (Variables|Default|GetFlashlightUI) "Collapsed")
  (Utilities|Time|PauseTimerbyHandle (Variables|Default|GetTimeHandleLoosingBattery))
  (Utilities|Time|PauseTimerbyHandle (Variables|Default|GetTimeHandlerChargingBattery)))

(event Event4thEquipmentAbility
  (Variables|Default|SetisCharging false)
  (Utilities|Time|PauseTimerbyHandle (Variables|Default|GetTimeHandlerChargingBattery))
  (if (not (== (Variables|Default|GetCurrentBattery) 0.0))
    (Rendering|SetVisibility (Variables|Default|GetSpotLight) true false)
    (Rendering|SetVisibility (Variables|Default|GetRevealCollision) true false)
    (CallFunction|TurnonLightCollision)
    (Utilities|Time|SetTimerbyFunctionName 0 "Loosing Battery" (Variables|Default|GetReduceBattery))))

(fn ConstructionScript
  (|CallParentFunction))

(fn SetUpWidgets
  (bind _returnvalue (UserInterface|CreateWidget "/Game/Blueprints/LvL_TheFlashight/Widgets/BW_FlashlightUI.BW_FlashlightUI_C"))
  (bind _output_get (Variables|Default|SetFlashlightUI _returnvalue))
  (UserInterface|Viewport|AddtoViewport _output_get 0)
  (Class|BIUpdateUI|UpdateUI(Message) _output_get (/ (Variables|Default|GetCurrentBattery) (Variables|Default|GetMaxBattery)))
  (Widget|SetVisibility (Variables|Default|GetFlashlightUI) "Collapsed"))

(fn ShootBullet
  (bind _bulletspawn (Variables|Default|GetBulletSpawn))
  (Game|SpawnActorfromClass "/Game/Blueprints/Test/BP_FlashlightBullet.BP_FlashlightBullet_C" (Math|Transform|MakeTransform (Transformation|GetWorldLocation _bulletspawn) (Transformation|GetWorldRotation _bulletspawn)) "Undefined" "MultiplyWithRoot" 0 0))

(fn TurnOffLightCollision
  (Collision|SetCollisionEnabled (Variables|Default|GetRevealCollision) "NoCollision"))

(fn TurnonLightCollision
  (Collision|SetCollisionEnabled (Variables|Default|GetRevealCollision) "QueryOnly"))