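; BP_Equipment is a base Blueprint for equipment that can be picked up and carried.
; On BeginPlay it creates a hidden viewport widget from a configurable class, then calls a 2ndBeginPlay hook.
; Interact disables the object's physics and collision and shows the widget, while Uninteract reverses this.
; Both update the PickedUp state and call empty PickedUp or Dropped events as extension points for specific equipment.
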(event Custom|Picked%20Up
  ;[1 0.1267 0.4822] What every equipment share in common to be able to be picked up and carried
)

(event Custom|Dropped
  ;[1 0.1267 0.4822] What every equipment share in common to be able to be picked up and carried
)

(event Custom|2ndBeginPlay
  ;[0.5672 0.2872 1] To be able to just drag and drop the right widget for the right Equipment further down the road and not do it the same setting up widget process through blueprints every time
)

(event EventUninteract
  (bind _widgetui_ref (Variables|Default|GetWidgetUI_Ref))
  (bind _object (Variables|Default|GetObject))
  ;[1 0.1267 0.4822] What every equipment share in common to be able to be picked up and carried
  (Physics|SetSimulatePhysics _object true)
  (Collision|SetCollisionEnabled _object "QueryAndPhysics")
  (Variables|Default|SetpickedUp false)
  (Utilities|IsValid _widgetui_ref
    (:Is%20Valid
      (Widget|SetVisibility _widgetui_ref "Collapsed"))
    (:Is%20Not%20Valid
      _))
  (CallFunction|Dropped))

(event EventBeginPlay
  ;[0.5672 0.2872 1] To be able to just drag and drop the right widget for the right Equipment further down the road and not do it the same setting up widget process through blueprints every time
  (CallFunction|SettingUpWidget)
  (CallFunction|2ndBeginPlay))

(event EventInteract
  (bind _widgetui_ref (Variables|Default|GetWidgetUI_Ref))
  (bind _object (Variables|Default|GetObject))
  ;[1 0.1267 0.4822] What every equipment share in common to be able to be picked up and carried
  (Physics|SetSimulatePhysics _object false)
  (Collision|SetCollisionEnabled _object "NoCollision")
  (Variables|Default|SetpickedUp true)
  (Utilities|IsValid _widgetui_ref
    (:Is%20Valid
      (Widget|SetVisibility _widgetui_ref "Visible"))
    (:Is%20Not%20Valid
      _))
  (CallFunction|PickedUp))

(fn ConstructionScript
  (|CallParentFunction))

(fn SettingUpWidget
  (bind _widgetref (Variables|Default|GetWidgetRef))
  (if (Utilities|IsValidClass _widgetref)
    (bind _returnvalue (UserInterface|CreateWidget _widgetref))
    (bind _output_get (Variables|Default|SetWidgetUI_Ref _returnvalue))
    (UserInterface|Viewport|AddtoViewport _output_get 0)
    (Widget|SetVisibility (Variables|Default|GetWidgetUI_Ref) "Collapsed")))