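; Test actor for an object whose material fade and collision respond to light, becoming passable while lit by the flashlight or other light spheres.
; Reveal and Hide track those sources, playing or reversing a Timeline that drives a dynamic material's Fade parameter.
; Collision toggles by switching object type between a custom channel and WorldDynamic.
; A SafePassage overlap delays restoration until the first-person character has left and no light remains.
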(event OnComponentBeginOverlap(SafePassage)
  (params (OverlappedComponent :type Primitive%20Component%20Object%20Reference) (OtherActor :type Actor%20Object%20Reference) (OtherComp :type Primitive%20Component%20Object%20Reference) (OtherBodyIndex :type Integer) (bFromSweep :type Boolean) (SweepResult :type Hit%20Result%20Structure%20%28by%20ref%29))
  (if (== (Utilities|GetClass OtherActor) "/Game/FirstPerson/Blueprints/BP_FirstPersonCharacter.BP_FirstPersonCharacter_C")
    (Utilities|Array|AddUnique (Variables|Default|GetObjectGoingThrough) OtherActor)))

(event OnComponentEndOverlap(SafePassage)
  (params (OverlappedComponent :type Primitive%20Component%20Object%20Reference) (OtherActor :type Actor%20Object%20Reference) (OtherComp :type Primitive%20Component%20Object%20Reference) (OtherBodyIndex :type Integer))
  (bind _maxfadevalue (Variables|Default|GetMaxFadeValue))
  (if (== (Utilities|GetClass OtherActor) "/Game/FirstPerson/Blueprints/BP_FirstPersonCharacter.BP_FirstPersonCharacter_C")
    (Utilities|Array|RemoveItem (Variables|Default|GetObjectGoingThrough) OtherActor)
    (if (not (or (Utilities|Array|IsValidIndex (Variables|Default|GetIsInLightArray)) (Utilities|IsValid (Variables|Default|GetFlashlightsLight))))
      (CallFunction|TurnonCollision)
      (bind _value (Timeline|Timeline Reverse)
        (:Update
          (Rendering|Material|SetScalarParameterValue (Variables|Default|GetFadeMaterial) "Fade" (Math|Float|Clamp(Float) (Math|Float|Lerp 0.0 _maxfadevalue _value) 0.0 _maxfadevalue) :!class /Script/Engine.MaterialInstanceDynamic)
          (Variables|Default|SetFadeValue (Math|Float|Clamp(Float) (Math|Float|Lerp 0.0 _maxfadevalue _value) 0.0 _maxfadevalue)))))))

(event EventBeginPlay
  (CallFunction|SettingUpFadeMaterial)
  (Transformation|SetWorldLocation (Variables|Default|GetNoise) (Transformation|GetWorldLocation (Variables|Default|GetObject)) false false)
  (Transformation|SetWorldLocation (Variables|Default|GetSafePassage) (Transformation|GetWorldLocation (Variables|Default|GetObject)) false false))

(event EventReveal
  (params (Component :type Static%20Mesh%20Component%20Object%20Reference) (SphereCollision :type Sphere%20Component%20Object%20Reference))
  (bind _isinlightarray (Variables|Default|GetIsInLightArray))
  (bind _maxfadevalue (Variables|Default|GetMaxFadeValue))
  (if (Utilities|IsValid Component)
    (Variables|Default|SetFlashlightsLight Component)
    (CallFunction|TurnOffCollision :!label _label)
    (bind _value (Timeline|Timeline Play)
      (:Update
        (Rendering|Material|SetScalarParameterValue (Variables|Default|GetFadeMaterial) "Fade" (Math|Float|Clamp(Float) (Math|Float|Lerp 0.0 _maxfadevalue _value) 0.0 _maxfadevalue) :!class /Script/Engine.MaterialInstanceDynamic)
        (Variables|Default|SetFadeValue (Math|Float|Clamp(Float) (Math|Float|Lerp 0.0 _maxfadevalue _value) 0.0 _maxfadevalue))))
    (else
      (Utilities|Array|AddUnique _isinlightarray SphereCollision)
      (if (Utilities|Array|IsValidIndex _isinlightarray)
        (goto _label)))))

(event EventHide
  (params (Component :type Static%20Mesh%20Component%20Object%20Reference) (SphereCollision :type Sphere%20Component%20Object%20Reference))
  (bind _isinlightarray (Variables|Default|GetIsInLightArray))
  (bind _maxfadevalue (Variables|Default|GetMaxFadeValue))
  (Utilities|IsValid Component
    (:Is%20Valid
      (if (Utilities|Enum|Equal(Enum) (Utilities|GetObjectName Component) (Utilities|GetObjectName (Variables|Default|GetFlashlightsLight)))
        (Variables|Default|SetFlashlightsLight 0)
        (if (not (Utilities|Array|IsValidIndex _isinlightarray)) :!label _label
          (if (not (Utilities|Array|IsValidIndex (Variables|Default|GetObjectGoingThrough)))
            (CallFunction|TurnonCollision)
            (bind _value (Timeline|Timeline Reverse)
              (:Update
                (Rendering|Material|SetScalarParameterValue (Variables|Default|GetFadeMaterial) "Fade" (Math|Float|Clamp(Float) (Math|Float|Lerp 0.0 _maxfadevalue _value) 0.0 _maxfadevalue) :!class /Script/Engine.MaterialInstanceDynamic)
                (Variables|Default|SetFadeValue (Math|Float|Clamp(Float) (Math|Float|Lerp 0.0 _maxfadevalue _value) 0.0 _maxfadevalue))))))))
    (:Is%20Not%20Valid
      (Utilities|Array|RemoveItem _isinlightarray SphereCollision)
      (Utilities|IsValid (Variables|Default|GetFlashlightsLight)
        (:Is%20Not%20Valid
          (goto _label))))))

(event EventTick
  (params (DeltaSeconds :type Float%20%28single-precision%29))
  (Development|PrintString (Utilities|GetObjectName (Variables|Default|GetFlashlightsLight))))

(fn ConstructionScript)

(fn SettingUpFadeMaterial
  (bind _returnvalue (Rendering|Material|CreateDynamicMaterialInstance "/Game/Materials/Material/FadeMaterial.FadeMaterial" "Fade" "None" :!class /Script/Engine.KismetMaterialLibrary))
  (bind _output_get (Variables|Default|SetFadeMaterial _returnvalue))
  (Rendering|Material|SetMaterial (Variables|Default|GetObject) 0 _output_get)
  (Rendering|Material|SetScalarParameterValue _output_get "Fade" 9e+01 :!class /Script/Engine.MaterialInstanceDynamic))

(fn TurnOffCollision
  (Collision|SetCollisionObjectType (Variables|Default|GetObject) "ECC_GameTraceChannel3"))

(fn TurnonCollision
  (Collision|SetCollisionObjectType (Variables|Default|GetObject) "ECC_WorldDynamic"))