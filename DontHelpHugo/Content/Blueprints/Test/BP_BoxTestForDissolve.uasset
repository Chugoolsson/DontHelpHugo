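; Test actor that feeds a box volume's transform to materials for a dissolve effect.
; The construction script writes the Box component's world location, scale and three axis vectors into the PC_DissolveTest2 parameter collection, defining an oriented box.
; The event graph holds an unconnected copy of the same writes and an empty Tick, so nothing updates the values during play.
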(event EventBeginPlay)

(event Collision|EventActorBeginOverlap
  (params (OtherActor :type Actor%20Object%20Reference)))

(event EventTick
  (params (DeltaSeconds :type Float%20%28single-precision%29)))

(fn ConstructionScript
  (bind _box (Variables|Default|GetBox))
  (bind _box_2 (Variables|Default|GetBox))
  (Rendering|Material|SetVectorParameterValue "/Game/Materials/Material/PC_DissolveTest2.PC_DissolveTest2" "Location" (Math|Conversions|ToLinearColor(Vector) (Transformation|GetWorldLocation _box)) :!class /Script/Engine.KismetMaterialLibrary)
  (Rendering|Material|SetVectorParameterValue "/Game/Materials/Material/PC_DissolveTest2.PC_DissolveTest2" "Bounds" (Math|Conversions|ToLinearColor(Vector) (Transformation|GetWorldScale _box)) :!class /Script/Engine.KismetMaterialLibrary)
  (Rendering|Material|SetVectorParameterValue "/Game/Materials/Material/PC_DissolveTest2.PC_DissolveTest2" "X" (Math|Conversions|ToLinearColor(Vector) (Math|Vector|GetForwardVector _box_2)) :!class /Script/Engine.KismetMaterialLibrary)
  (Rendering|Material|SetVectorParameterValue "/Game/Materials/Material/PC_DissolveTest2.PC_DissolveTest2" "Y" (Math|Conversions|ToLinearColor(Vector) (Math|Vector|GetRightVector _box_2)) :!class /Script/Engine.KismetMaterialLibrary)
  (Rendering|Material|SetVectorParameterValue "/Game/Materials/Material/PC_DissolveTest2.PC_DissolveTest2" "Z" (Math|Conversions|ToLinearColor(Vector) (Math|Vector|GetUpVector _box_2)) :!class /Script/Engine.KismetMaterialLibrary))