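; Test parent Blueprint for interactable objects that toggle their look and can alert actors that come within their noise volume.
; On BeginPlay it snaps the Noise and Sphere components to the Object component's world location.
; Any actor that begins overlapping Noise receives a HeardSomething message, independent of interaction.
; The Interact event uses a FlipFlop to alternate Object's material between the projectile and base materials.
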(event OnComponentBeginOverlap(Noise)
  (params (OverlappedComponent :type Primitive%20Component%20Object%20Reference) (OtherActor :type Actor%20Object%20Reference) (OtherComp :type Primitive%20Component%20Object%20Reference) (OtherBodyIndex :type Integer) (bFromSweep :type Boolean) (SweepResult :type Hit%20Result%20Structure%20%28by%20ref%29))
  ;[0.5016 0.8164 1] First Interactable BP parent
  (Class|BIHearing|HeardSomething(Message) OtherActor))

(event EventBeginPlay
  ;[0.5016 0.8164 1] First Interactable BP parent
  (Transformation|SetWorldLocation (Variables|Default|GetNoise) (Transformation|GetWorldLocation (Variables|Default|GetObject)) false false)
  (Transformation|SetWorldLocation (Variables|Default|GetSphere) (Transformation|GetWorldLocation (Variables|Default|GetObject)) false false))

(event EventInteract
  (bind _object (Variables|Default|GetObject))
  ;[0.5016 0.8164 1] First Interactable BP parent
  (Utilities|FlowControl|FlipFlop
    (:A
      (Rendering|Material|SetMaterial _object 0 "/Game/FPWeapon/Materials/FirstPersonProjectileMaterial.FirstPersonProjectileMaterial"))
    (:B
      (Rendering|Material|SetMaterial _object 0 "/Game/FPWeapon/Materials/BaseMaterial.BaseMaterial"))))

(fn ConstructionScript)