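; BP_FadeObject is a test actor that fades its object in and out as actors reveal or hide it, apparently tied to light.
; On BeginPlay it applies a dynamic material instance to the object with the Fade parameter at zero.
; Reveal and Hide events track the calling actors in IsInLightArray.
; A timeline drives Fade forward while any actor is listed and reverses once the array empties, so overlapping sources coexist.
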(event Custom|Hide_1_1
  (params (Actor :type Actor%20Object%20Reference))
  (bind _isinlightarray (Variables|Default|GetisInLightArray))
  (Utilities|Array|RemoveItem _isinlightarray Actor)
  (if (not (Utilities|Array|IsValidIndex _isinlightarray))
    (bind _value (Timeline|RevealTimeline Reverse)
      (:Update
        (Rendering|Material|SetScalarParameterValue (Variables|Default|GetFadeMaterial) "Fade" _value :!class /Script/Engine.MaterialInstanceDynamic)))))

(event Custom|Reveal_1_1
  (params (Actor :type Actor%20Object%20Reference))
  (bind _isinlightarray (Variables|Default|GetisInLightArray))
  (Utilities|Array|AddUnique _isinlightarray Actor)
  (if (Utilities|Array|IsValidIndex _isinlightarray)
    (bind _value (Timeline|RevealTimeline Play)
      (:Update
        (Rendering|Material|SetScalarParameterValue (Variables|Default|GetFadeMaterial) "Fade" _value :!class /Script/Engine.MaterialInstanceDynamic)))))

(event EventBeginPlay
  (bind _returnvalue (Rendering|Material|CreateDynamicMaterialInstance "/Game/Materials/Material/FadeMaterial.FadeMaterial" "Fade" "None" :!class /Script/Engine.KismetMaterialLibrary))
  (bind _output_get (Variables|Default|SetFadeMaterial _returnvalue))
  (Rendering|Material|SetMaterial (Variables|Default|GetObject) 0 _output_get)
  (Rendering|Material|SetScalarParameterValue _output_get "Fade" 0.0 :!class /Script/Engine.MaterialInstanceDynamic))

(fn ConstructionScript)

(fn Hide
  (params (Actor :type Actor%20Object%20Reference))
  (return 0))

(fn Reveal
  (params (Actor :type Actor%20Object%20Reference))
  (return 0))