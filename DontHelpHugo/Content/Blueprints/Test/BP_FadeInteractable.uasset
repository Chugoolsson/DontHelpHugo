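; Test interactable that fades its object in when lit, starting at zero Fade and ignoring the Visibility channel.
; Reveal makes it block Visibility and plays a timeline driving a dynamic material's Fade, tracking non-flashlight light spheres in an array.
; Hide removes the sphere and immediately ignores Visibility, but reverses the fade only when the array is empty.
; Two helper functions set Visibility to Ignore or Overlap.
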(event EventReveal
  (params (Component :type Static%20Mesh%20Component%20Object%20Reference) (SphereCollision :type Sphere%20Component%20Object%20Reference))
  (bind _isinlightarray (Variables|Default|GetisInLightArray))
  (if (== (Utilities|GetClass Component) "/Game/Blueprints/Test/BP_TestFlshlight.BP_TestFlshlight_C")
    (Collision|SetCollisionResponsetoChannel (Variables|Default|GetObject) "ECC_Visibility" "ECR_Block" :!label _label)
    (bind _value (Timeline|Timeline Play)
      (:Update
        (Rendering|Material|SetScalarParameterValue (Variables|Default|GetFadeMaterial) "Fade" _value :!class /Script/Engine.MaterialInstanceDynamic)))
    (else
      (Utilities|Array|AddUnique _isinlightarray SphereCollision)
      (if (Utilities|Array|IsValidIndex _isinlightarray)
        (goto _label)))))

(event EventHide
  (params (Component :type Static%20Mesh%20Component%20Object%20Reference) (SphereCollision :type Sphere%20Component%20Object%20Reference))
  (bind _isinlightarray (Variables|Default|GetisInLightArray))
  (Utilities|Array|RemoveItem _isinlightarray SphereCollision)
  (Collision|SetCollisionResponsetoChannel (Variables|Default|GetObject) "ECC_Visibility" "ECR_Ignore")
  (if (not (Utilities|Array|IsValidIndex _isinlightarray))
    (bind _value (Timeline|Timeline Reverse)
      (:Update
        (Rendering|Material|SetScalarParameterValue (Variables|Default|GetFadeMaterial) "Fade" _value :!class /Script/Engine.MaterialInstanceDynamic)))))

(event EventBeginPlay
  (CallFunction|DynamicMaterialSetUp)
  (Collision|SetCollisionResponsetoChannel (Variables|Default|GetObject) "ECC_Visibility" "ECR_Ignore"))

(fn ConstructionScript
  (|CallParentFunction))

(fn DynamicMaterialSetUp
  (bind _returnvalue (Rendering|Material|CreateDynamicMaterialInstance "/Game/Materials/Material/FadeMaterial.FadeMaterial" "Fade" "None" :!class /Script/Engine.KismetMaterialLibrary))
  (bind _output_get (Variables|Default|SetFadeMaterial _returnvalue))
  (Rendering|Material|SetMaterial (Variables|Default|GetObject) 0 _output_get)
  (Rendering|Material|SetScalarParameterValue _output_get "Fade" 0.0 :!class /Script/Engine.MaterialInstanceDynamic))

(fn IgonerPlayerLineTrace
  (Collision|SetCollisionResponsetoChannel (Variables|Default|GetObject) "ECC_Visibility" "ECR_Ignore"))

(fn NoticePlayerLineTrace
  (Collision|SetCollisionResponsetoChannel (Variables|Default|GetObject) "ECC_Visibility" "ECR_Overlap"))