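; BP_FlashlightBullet1 is a temporary glowing light source that reveals hidden messages on actors inside its trigger sphere.
; Overlap begin and end call RevealMessage and HideMessage via CBP_Reveal, falling back to the BI_Reveal interface.
; After a delay timeline, a second timeline animates the dynamic material glow, light intensity, trigger radius and revealer scale.
; When it finishes, the light components are destroyed and the object simulates physics, also triggerable through RemoveStuckedObject.
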(event OnComponentBeginOverlap(LightTrigger)
  (params (OverlappedComponent :type Primitive%20Component%20Object%20Reference) (OtherActor :type Actor%20Object%20Reference) (OtherComp :type Primitive%20Component%20Object%20Reference) (OtherBodyIndex :type Integer) (bFromSweep :type Boolean) (SweepResult :type Hit%20Result%20Structure%20%28by%20ref%29))
  (bind _returnvalue (Actor|GetComponentbyClass OtherActor "/Game/Blueprints/LvL_TheFlashight/Actor_Components/CBP_Reveal.CBP_Reveal_C"))
  (Utilities|IsValid _returnvalue
    (:Is%20Valid
      (Class|BIReveal|Reveal(Message) _returnvalue))
    (:Is%20Not%20Valid
      (if (Utilities|DoesObjectImplementInterface OtherActor "/Game/Blueprints/LvL_TheFlashight/Interfaces/BI_Reveal.BI_Reveal_C")
        (Class|BIReveal|Reveal(Message) OtherActor)))))

(event OnComponentEndOverlap(LightTrigger)
  (params (OverlappedComponent :type Primitive%20Component%20Object%20Reference) (OtherActor :type Actor%20Object%20Reference) (OtherComp :type Primitive%20Component%20Object%20Reference) (OtherBodyIndex :type Integer))
  (bind _returnvalue (Actor|GetComponentbyClass OtherActor "/Game/Blueprints/LvL_TheFlashight/Actor_Components/CBP_Reveal.CBP_Reveal_C"))
  (Utilities|IsValid _returnvalue
    (:Is%20Valid
      (Class|BIReveal|Hide(Message) _returnvalue))
    (:Is%20Not%20Valid
      (if (Utilities|DoesObjectImplementInterface OtherActor "/Game/Blueprints/LvL_TheFlashight/Interfaces/BI_Reveal.BI_Reveal_C")
        (Class|BIReveal|Hide(Message) OtherActor)))))

(event Custom|TimeLineToCountDown
  (Timeline|TimelineToStartLifeSpan Play
    (:Finished
      (CallFunction|LifeSpan))))

(event Custom|LifeSpan
  (bind (_direction _emissiceglowvalue _lightintensity _lightcollisionsize _set__light__revealer_size) (Timeline|LifeSpanCountDown Play)
    (:Update
      (Rendering|Material|SetScalarParameterValue (Variables|Default|GetEmissiveValueMaterial) "Glow" _emissiceglowvalue :!class /Script/Engine.MaterialInstanceDynamic)
      (Rendering|Components|Light|SetIntensity (Variables|Default|GetPointLight) _lightintensity)
      (Components|Sphere|SetSphereRadius (Variables|Default|GetLightTrigger) _lightcollisionsize true)
      (Transformation|SetRelativeScale3D (Variables|Default|GetLightRevealer) _set__light__revealer_size))
    (:Finished
      (CallFunction|Death))))

(event Custom|Death
  (Components|DestroyComponent (Variables|Default|GetPointLight))
  (Components|DestroyComponent (Variables|Default|GetLightTrigger))
  (Components|DestroyComponent (Variables|Default|GetLightRevealer))
  (Physics|SetSimulatePhysics (Variables|Default|GetObject) true))

(event EventRemoveStuckedObject
  (Physics|SetSimulatePhysics (Variables|Default|GetObject) true))

(event EventBeginPlay
  (CallFunction|TimeLinetoCountDown)
  (CallFunction|CreateDynamicMaterial)
  (Components|Sphere|SetSphereRadius (Variables|Default|GetLightTrigger) 25.0 true))

(fn ConstructionScript)

(fn CreateDynamicMaterial
  (bind _returnvalue (Rendering|Material|CreateDynamicMaterialInstance "/Game/Materials/Material/Colors/MI_EmissiveWhite.MI_EmissiveWhite" "Glow" "None" :!class /Script/Engine.KismetMaterialLibrary))
  (bind _output_get (Variables|Default|SetEmissiveValueMaterial _returnvalue))
  (Rendering|Material|SetMaterial (Variables|Default|GetObject) 0 _output_get)
  (Rendering|Material|SetScalarParameterValue _output_get "Glow" 5.0 :!class /Script/Engine.MaterialInstanceDynamic))