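; Test Blueprint that acts as a repeating noise source for AI hearing.
; From BeginPlay, the Noise event reports a short-range noise event at its location with itself as instigator and spawns an explosion emitter just above it.
; Noise re-arms a non-looping timer on itself to repeat every few seconds.
; Alternative MakeNoise calls, including one through a PawnNoiseEmitter, are left unconnected and never run.
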(event Custom|Noise
  (bind _self self)
  (Class|AISenseHearing|ReportNoiseEvent (Transformation|GetActorLocation _self) 1.0 _self 4e+02 "None")
  (Utilities|Time|SetTimerbyEvent (delegate Custom|Noise) 1e+01)
  (Effects|SpawnEmitteratLocation "/Game/StarterContent/Particles/P_Explosion.P_Explosion" (+ (Transformation|GetActorLocation) "0.000000,0.000000,50.000000")))

(event EventBeginPlay
  (CallFunction|Noise))

(fn ConstructionScript)