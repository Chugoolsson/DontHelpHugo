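; Base enemy Blueprint in a test AI folder that caches its AI_BaseController on BeginPlay.
; When another base enemy leaves its proximity collision, it decrements a nearby count and clears the FellowEnemiesNearby blackboard key at zero; no increment appears here.
; Perception and Tick events are empty.
; Unconnected leftover logic would switch controller states between patrolling, seeing the player, in light and investigating, based on sight and flashlight exposure.
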(event OnComponentEndOverlap(NearOtherEnemyCollision)
  (params (OverlappedComponent :type Primitive%20Component%20Object%20Reference) (OtherActor :type Actor%20Object%20Reference) (OtherComp :type Primitive%20Component%20Object%20Reference) (OtherBodyIndex :type Integer))
  (bind _fellowenemiesnearbycount (Variables|Default|GetFellowEnemiesNearbyCount))
  (if (== (Utilities|GetClass OtherActor) "BP_BaseEnemy_C")
    (Math|Integer|DecrementInt _fellowenemiesnearbycount
      (:%20%20
        (if (<= _fellowenemiesnearbycount 0)
          (AI|Components|Blackboard|SetValueasBool (AI|GetBlackboard (AI|GetAIController self)) (Utilities|Name|MakeLiteralName "FellowEnemiesNearby") false))))))

(event OnTargetPerceptionUpdated(AIPerception)
  (params (Actor :type Actor%20Object%20Reference) (Stimulus :type AI%20Stimulus%20Structure)))

(event EventTick
  (params (DeltaSeconds :type Float%20%28single-precision%29)))

(event EventBeginPlay
  (bind _asai_base_controller (Utilities|Casting|CastToAI_BaseController (AI|GetAIController self)))
  (Variables|Default|SetAIBaseController _asai_base_controller))

(fn ConstructionScript)