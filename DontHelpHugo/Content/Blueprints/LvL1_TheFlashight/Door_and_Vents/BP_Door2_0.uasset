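; BP_Door2_0 is a swinging door that players open through Interact and enemies trigger by entering its sphere.
; At BeginPlay it moves an anchor to the mesh edge as a hinge and reparents the door.
; A side-collision counter picks the swing direction for a randomly delayed timeline rotation, which reverses when characters leave the sphere.
; It releases stuck flashlight bullets before moving; Tick prints the counter for debugging.
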(event OnComponentBeginOverlap(Side_A_Collision)
  (params (OverlappedComponent :type Primitive%20Component%20Object%20Reference) (OtherActor :type Actor%20Object%20Reference) (OtherComp :type Primitive%20Component%20Object%20Reference) (OtherBodyIndex :type Integer) (bFromSweep :type Boolean) (SweepResult :type Hit%20Result%20Structure%20%28by%20ref%29))
  (bind _returnvalue (Utilities|GetClass OtherActor))
  ;[0.7435 0.2539 1] Setting up to see which side of the door the player is on
  (if (or (== _returnvalue "/Game/FirstPerson/Blueprints/BP_FirstPersonCharacter.BP_FirstPersonCharacter_C") (== _returnvalue "/Game/Blueprints/Test/AI/BP_BaseEnemy.BP_BaseEnemy_C"))
    (Math|Integer|IncrementInt (Variables|Default|GetSideA))))

(event OnComponentEndOverlap(Side_A_Collision)
  (params (OverlappedComponent :type Primitive%20Component%20Object%20Reference) (OtherActor :type Actor%20Object%20Reference) (OtherComp :type Primitive%20Component%20Object%20Reference) (OtherBodyIndex :type Integer))
  (bind _returnvalue (Utilities|GetClass OtherActor))
  ;[0.7435 0.2539 1] Setting up to see which side of the door the player is on
  (if (or (== _returnvalue "/Game/FirstPerson/Blueprints/BP_FirstPersonCharacter.BP_FirstPersonCharacter_C") (== _returnvalue "/Game/Blueprints/Test/AI/BP_BaseEnemy.BP_BaseEnemy_C"))
    (bind _result (Math|Integer|DecrementInt (Variables|Default|GetSideA))
      (:%20%20
        (Variables|Default|SetSideA (Math|Integer|Clamp(Integer) _result 0 5))))))

(event OnComponentEndOverlap(Sphere)
  (params (OverlappedComponent :type Primitive%20Component%20Object%20Reference) (OtherActor :type Actor%20Object%20Reference) (OtherComp :type Primitive%20Component%20Object%20Reference) (OtherBodyIndex :type Integer))
  (bind _returnvalue (Utilities|GetClass OtherActor))
  (bind _sphere (Variables|Default|GetSphere))
  ;[1 0.1571 0.4486] Opening and closing the door. Door opens away from the player
  (if (and (Variables|Default|GetIsOpen) (or (== _returnvalue "/Game/FirstPerson/Blueprints/BP_FirstPersonCharacter.BP_FirstPersonCharacter_C") (== _returnvalue "/Game/Blueprints/Test/AI/BP_BaseEnemy.BP_BaseEnemy_C")))
    (for _array_element (Variables|Default|GetStuckedObjects)
      ;;[1 0.1167 0] In case some "Flashlight Bullets" has gotten stuck on the door.
      (Class|BISomethingIsStuckonYou|RemoveStuckedObject(Message) _array_element))
    (bind _alpha (Timeline|RotatingDoor Reverse)
      (:Update
        (Transformation|SetRelativeRotation (Variables|Default|GetANCHOR) (Math|Rotator|Lerp(Rotator) (Variables|Default|GetCurrentRotation) (Variables|Default|GetRotateDestination) _alpha) false false))
      (:Finished
        (if (<= _alpha 0.2)
          (Variables|Default|SetIsOpen false)
          (Collision|SetCollisionResponsetoChannel (Variables|Default|GetDoor) "ECC_Visibility" "ECR_Block")
          (elif (not (or (Utilities|Array|IsValidIndex (Collision|GetOverlappingActors _sphere "/Game/FirstPerson/Blueprints/BP_FirstPersonCharacter.BP_FirstPersonCharacter_C" :!class /Script/Engine.PrimitiveComponent)) (Utilities|Array|IsValidIndex (Collision|GetOverlappingActors _sphere "/Game/Blueprints/Test/AI/BP_BaseEnemy.BP_BaseEnemy_C" :!class /Script/Engine.PrimitiveComponent))))
            (Timeline|RotatingDoor Reverse)))))))

(event OnComponentBeginOverlap(Sphere)
  (params (OverlappedComponent :type Primitive%20Component%20Object%20Reference) (OtherActor :type Actor%20Object%20Reference) (OtherComp :type Primitive%20Component%20Object%20Reference) (OtherBodyIndex :type Integer) (bFromSweep :type Boolean) (SweepResult :type Hit%20Result%20Structure%20%28by%20ref%29))
  (if (and (== (Utilities|GetClass OtherActor) "/Game/Blueprints/Test/AI/BP_BaseEnemy.BP_BaseEnemy_C") (!= (Variables|Default|GetIsOpen) true))
    (CallFunction|Interact)))

(event EventBeginPlay
  (bind _rotatingdoor (Variables|Default|GetRotatingDoor))
  ;[0.4429 0.2826 1] Setting up and changing parent to anchor for later rotation
  (CallFunction|SettingUpAnchorasParrent)
  (Components|Timeline|SetPlayRate _rotatingdoor (/ (Components|Timeline|GetTimelineLength _rotatingdoor) (Variables|Default|GetTimeToRotate))))

(event EventInteract
  (bind _sphere (Variables|Default|GetSphere))
  ;[1 0.1571 0.4486] Opening and closing the door. Door opens away from the player
  (Variables|Default|SetIsOpen true)
  (Collision|SetCollisionResponsetoChannel (Variables|Default|GetDoor) "ECC_Visibility" "ECR_Ignore")
  (Variables|Default|SetCurrentRotation (Variables|/Script/Engine.SceneComponent|GetRelativeRotation (Variables|Default|GetANCHOR)))
  (if (== (Variables|Default|GetSideA) 0)
    (Variables|Default|SetRotateDestination (Math|Rotator|MakeRotator 0.0 0.0 (+ (.yaw (Variables|Default|GetCurrentRotation)) -9e+01)))
    (else
      (Variables|Default|SetRotateDestination (Math|Rotator|MakeRotator 0.0 0.0 (+ (.yaw (Variables|Default|GetCurrentRotation)) 9e+01)))))
  (Utilities|FlowControl|Delay (Math|Random|RandomFloatinRange (Variables|Default|GetMinimumTimeToStartRotate) (Variables|Default|GetMaximumTimeToStartRotate)))
  (for _array_element (Variables|Default|GetStuckedObjects)
    ;;[1 0.1167 0] In case some "Flashlight Bullets" has gotten stuck on the door.
    (Class|BISomethingIsStuckonYou|RemoveStuckedObject(Message) _array_element))
  (bind _alpha (Timeline|RotatingDoor Play)
    (:Update
      (Transformation|SetRelativeRotation (Variables|Default|GetANCHOR) (Math|Rotator|Lerp(Rotator) (Variables|Default|GetCurrentRotation) (Variables|Default|GetRotateDestination) _alpha) false false))
    (:Finished
      (if (<= _alpha 0.2)
        (Variables|Default|SetIsOpen false)
        (Collision|SetCollisionResponsetoChannel (Variables|Default|GetDoor) "ECC_Visibility" "ECR_Block")
        (elif (not (or (Utilities|Array|IsValidIndex (Collision|GetOverlappingActors _sphere "/Game/FirstPerson/Blueprints/BP_FirstPersonCharacter.BP_FirstPersonCharacter_C" :!class /Script/Engine.PrimitiveComponent)) (Utilities|Array|IsValidIndex (Collision|GetOverlappingActors _sphere "/Game/Blueprints/Test/AI/BP_BaseEnemy.BP_BaseEnemy_C" :!class /Script/Engine.PrimitiveComponent))))
          (Timeline|RotatingDoor Reverse))))))

(event EventObjectGotStucked
  (params (StuckObject :type Actor%20Object%20Reference))
  (Utilities|Array|AddUnique (Variables|Default|GetStuckedObjects) StuckObject))

(event EventTick
  (params (DeltaSeconds :type Float%20%28single-precision%29))
  (Development|PrintString (Utilities|String|ToString(Integer) (Variables|Default|GetSideA))))

(fn ConstructionScript)

(fn SettingUpAnchorasParrent
  (bind _door (Variables|Default|GetDoor))
  (bind _anchor (Variables|Default|GetANCHOR))
  (bind _staticmesh (Variables|/Script/Engine.StaticMeshComponent|GetStaticMesh _door))
  (bind _returnvalue (StaticMesh|GetBoundingBox _staticmesh))
  (bind (_min _max) (Utilities|Struct|BreakBox _returnvalue))
  (Transformation|SetWorldLocation _anchor (- (Transformation|GetWorldLocation _anchor) (* (Math|Vector|GetRightVector _anchor) (/ (- (.y _max) (.y _min)) 2.0))) false false)
  (Transformation|AttachComponentToComponent (Variables|Default|GetDoor) (Variables|Default|GetANCHOR) "None" "KeepWorld" "KeepWorld" "KeepWorld" true))