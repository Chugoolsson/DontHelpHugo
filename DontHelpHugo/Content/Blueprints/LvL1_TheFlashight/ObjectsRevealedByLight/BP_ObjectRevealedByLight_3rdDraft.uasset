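; Base object for the flashlight level that grows from a minimum size to full scale when lit, hiding its counterpart body, and reverses when unlit.
; Reveal and Hide calls maintain a light-source count that drives a scale timeline.
; A SafePassage box, sized from mesh bounds, defers both transitions while the player is inside and re-evaluates on exit.
; Hiding also notifies registered stuck objects; an optional tag marks it interactible.
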(event OnComponentBeginOverlap(SafePassage)
  (params (OverlappedComponent :type Primitive%20Component%20Object%20Reference) (OtherActor :type Actor%20Object%20Reference) (OtherComp :type Primitive%20Component%20Object%20Reference) (OtherBodyIndex :type Integer) (bFromSweep :type Boolean) (SweepResult :type Hit%20Result%20Structure%20%28by%20ref%29))
  (if (and (== (Utilities|GetClass OtherActor) "/Game/FirstPerson/Blueprints/BP_FirstPersonCharacter.BP_FirstPersonCharacter_C") (Variables|ActorAbilities|GetisRevealedByLight))
    (Math|Integer|IncrementInt (Variables|ParentVariables|GetPlayerInSafePassage))))

(event OnComponentEndOverlap(SafePassage)
  (params (OverlappedComponent :type Primitive%20Component%20Object%20Reference) (OtherActor :type Actor%20Object%20Reference) (OtherComp :type Primitive%20Component%20Object%20Reference) (OtherBodyIndex :type Integer))
  (bind _playerinsafepassage (Variables|ParentVariables|GetPlayerInSafePassage))
  (if (Math|Boolean|ANDBoolean (== (Utilities|GetClass OtherActor) "/Game/FirstPerson/Blueprints/BP_FirstPersonCharacter.BP_FirstPersonCharacter_C") (not (== _playerinsafepassage 0)) (Variables|ActorAbilities|GetisRevealedByLight))
    (bind _result (Math|Integer|DecrementInt _playerinsafepassage)
      (:%20%20
        (if (and (== (Math|Integer|Clamp(Integer) _result 0 100) 0) (<= (Variables|ParentVariables|GetLightSources) 0))
          (CallFunction|LeftSafePassagewithZeroLightSOurcesonObject)
          (else
            (CallFunction|LeftSafePassagewithLightSourcesonObject)))))))

(event Custom|RevealingObjectWithTimer
  (bind _size (Timeline|RevealTimer Play)
    (:Update
      (Transformation|SetWorldScale3D (Variables|Default|GetObjectBodyToBeRevealed) (Math|Vector|Lerp(Vector) (Variables|ParentVariables|GetMinimumSize) (Variables|ParentVariables|GetOriginalObjectSize) _size)))
    (:Finished
      (if (>= _size 0.5)
        (CallFunction|DoneRevealingObject)
        (else
          (CallFunction|DoneHidingObject))))))

(event Custom|DoneRevealingObject
  (bind _objectbodytobehidden (Variables|Default|GetObjectBodyToBeHidden))
  (Development|SetHiddeninGame _objectbodytobehidden true false)
  (Collision|SetCollisionEnabled _objectbodytobehidden "NoCollision"))

(event Custom|HideObjectWithTimer
  (bind _size (Timeline|RevealTimer Reverse)
    (:Update
      (Transformation|SetWorldScale3D (Variables|Default|GetObjectBodyToBeRevealed) (Math|Vector|Lerp(Vector) (Variables|ParentVariables|GetMinimumSize) (Variables|ParentVariables|GetOriginalObjectSize) _size)))
    (:Finished
      (if (>= _size 0.5)
        (CallFunction|DoneRevealingObject)
        (else
          (CallFunction|DoneHidingObject))))))

(event Custom|DoneHidingObject)

(event Custom|RevealWithoutAddingLightSource
  (if (and (== (Variables|ParentVariables|GetLightSources) 1) (<= (Variables|ParentVariables|GetPlayerInSafePassage) 0))
    (CallFunction|RevealingObjectwithTimer)))

(event Custom|LeftSafePassageWithZeroLightSOurcesOnObject
  (CallFunction|Hide))

(event Custom|LeftSafePassageWithLightSourcesOnObject
  (CallFunction|RevealWithoutAddingLightSource))

(event EventBeginPlay
  (bind _revealtimer (Variables|Default|GetRevealTimer))
  (CallFunction|SettingUpInteract)
  (if (Variables|ActorAbilities|GetisRevealedByLight)
    (Variables|ParentVariables|SetOriginalObjectSize (Transformation|GetWorldScale (Variables|Default|GetObjectBodyToBeRevealed)))
    (Components|Timeline|SetPlayRate _revealtimer (/ (Components|Timeline|GetTimelineLength _revealtimer) (Variables|ParentVariables|GetRevealTimerPlayRate)))
    (CallFunction|SettingUpRevealandHideCheck)
    (CallFunction|SettingUpSafePassage)
    (Transformation|SetWorldScale3D (Variables|Default|GetObjectBodyToBeRevealed) (Variables|ParentVariables|GetMinimumSize))))

(event EventObjectGotStucked
  (params (StuckObject :type Actor%20Object%20Reference))
  (Utilities|Array|AddUnique (Variables|ParentVariables|GetStuckedObjects) StuckObject))

(event EventReveal
  (params (Component :type Static%20Mesh%20Component%20Object%20Reference) (SphereCollision :type Sphere%20Component%20Object%20Reference))
  (bind _lightsources (Variables|ParentVariables|GetLightSources))
  (if (Variables|ActorAbilities|GetisRevealedByLight)
    (Math|Integer|IncrementInt _lightsources
      (:%20%20
        (if (and (== _lightsources 1) (<= (Variables|ParentVariables|GetPlayerInSafePassage) 0))
          (CallFunction|RevealingObjectwithTimer))))))

(event EventHide
  (params (Component :type Static%20Mesh%20Component%20Object%20Reference) (SphereCollision :type Sphere%20Component%20Object%20Reference))
  (if (Variables|ActorAbilities|GetisRevealedByLight)
    (if (<= (Variables|ParentVariables|GetLightSources) 0)
      _
      (else
        (bind _output_get (CallFunction|SubtractLightSource))))
    (if (and (<= _output_get 0) (<= (Variables|ParentVariables|GetPlayerInSafePassage) 0))
      (CallFunction|HideObjectwithTimer)
      (Development|SetHiddeninGame (Variables|Default|GetObjectBodyToBeHidden) false false)
      (Collision|SetCollisionEnabled (Variables|Default|GetObjectBodyToBeHidden) "QueryAndPhysics")
      (for _array_element (Variables|ParentVariables|GetStuckedObjects)
        (Class|BISomethingIsStuckonYou|RemoveStuckedObject(Message) _array_element)))))

(fn ConstructionScript)

(fn SettingUpRevealandHideCheck
  (bind _objectbodytoberevealed (Variables|Default|GetObjectBodyToBeRevealed))
  (bind _staticmesh (Variables|/Script/Engine.StaticMeshComponent|GetStaticMesh _objectbodytoberevealed))
  (bind _returnvalue (StaticMesh|GetBoundingBox _staticmesh))
  (bind (_min _max) (Utilities|Struct|BreakBox _returnvalue))
  (Components|Box|SetBoxExtent (Variables|Default|GetRevealAndHideCheck) (/ (- _max _min) "2.000000,2.000000,2.000000") true))

(fn SettingUpSafePassage
  (bind _objectbodytoberevealed (Variables|Default|GetObjectBodyToBeRevealed))
  (bind _objectbodytobehidden (Variables|Default|GetObjectBodyToBeHidden))
  (bind _staticmesh (Variables|/Script/Engine.StaticMeshComponent|GetStaticMesh _objectbodytoberevealed))
  (bind _staticmesh_2 (Variables|/Script/Engine.StaticMeshComponent|GetStaticMesh _objectbodytobehidden))
  (bind _returnvalue (StaticMesh|GetBoundingBox _staticmesh))
  (bind _returnvalue_2 (StaticMesh|GetBoundingBox _staticmesh_2))
  (bind (_min _max) (Utilities|Struct|BreakBox _returnvalue))
  (bind (_min_2 _max_2) (Utilities|Struct|BreakBox _returnvalue_2))
  (Utilities|IsValid _staticmesh_2
    (:Is%20Valid
      (Components|Box|SetBoxExtent (Variables|Default|GetSafePassage) (/ (- _max_2 _min_2) "1.500000,1.500000,1.500000") true))
    (:Is%20Not%20Valid
      (Components|Box|SetBoxExtent (Variables|Default|GetSafePassage) (/ (- _max _min) "1.500000,1.500000,1.500000") true))))

(fn SettingUpInteract
  (if (Variables|ActorAbilities|GetisInteractible)
    (Utilities|Array|AddUnique (Variables|Actor|GetTags) (Variables|ParentVariables|GetInteractibleTagString))))

(fn SubtractLightSource
  (bind _output_get (Variables|ParentVariables|SetLightSources (Math|Integer|Clamp(Integer) (- (Variables|ParentVariables|GetLightSources) 1) 0 1000)))
  (return _output_get))