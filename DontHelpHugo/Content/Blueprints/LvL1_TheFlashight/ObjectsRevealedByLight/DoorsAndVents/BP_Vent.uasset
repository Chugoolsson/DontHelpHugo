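; Vent that is revealed by light and opens when the player interacts within its distance check, on top of inherited reveal/hide logic.
; Opening clears its reveal flag and trace blocking, removes stuck-object messages, then plays a timeline scaled to the open time.
; Leaving range mid-opening reverses the timeline; closing restores both and hides the vent if unlit.
; Tick prints the light-source count for debugging.
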(event OnComponentEndOverlap(OpeningDistanceCheck)
  (params (OverlappedComponent :type Primitive%20Component%20Object%20Reference) (OtherActor :type Actor%20Object%20Reference) (OtherComp :type Primitive%20Component%20Object%20Reference) (OtherBodyIndex :type Integer))
  (bind _openingventtimer (Variables|Default|GetOpeningVentTimer))
  (if (and (== (Utilities|GetClass OtherActor) "/Game/FirstPerson/Blueprints/BP_FirstPersonCharacter.BP_FirstPersonCharacter_C") (Audio|Components|Audio|IsPlaying (Variables|Default|GetOpeningVentTimer)))
    (bind _transformation (Timeline|OpeningVentTimer Reverse)
      (:Update
        (Transformation|SetRelativeLocation (Variables|Default|GetObjectBodyToBeRevealed) _transformation false false))
      (:Finished
        (if (not (> (Components|Timeline|GetPlaybackPosition _openingventtimer) (- (Components|Timeline|GetTimelineLength _openingventtimer) 0.5)))
          (CallFunction|Close))))))

(event Custom|Open
  (Variables|Default|SetisRevealedByLight false)
  (Collision|SetCollisionResponsetoChannel (Variables|Default|GetObjectBodyToBeRevealed) "ECC_GameTraceChannel2" "ECR_Ignore")
  (for _array_element (Variables|Default|GetStuckedObjects)
    (Class|BISomethingIsStuckonYou|RemoveStuckedObject(Message) _array_element))
  (CallFunction|StartMovingtobeOpen))

(event Custom|StartMovingToBeOpen
  (bind _objectbodytoberevealed (Variables|Default|GetObjectBodyToBeRevealed))
  (bind _openingventtimer (Variables|Default|GetOpeningVentTimer))
  (bind _returnvalue (Transformation|GetWorldLocation _objectbodytoberevealed))
  (Variables|Default|SetStartPos _returnvalue)
  (Variables|Default|SetEndPos (+ _returnvalue "20.000000,-130.000000,0.000000"))
  (bind _transformation (Timeline|OpeningVentTimer PlayFromStart)
    (:Update
      (Transformation|SetRelativeLocation (Variables|Default|GetObjectBodyToBeRevealed) _transformation false false))
    (:Finished
      (if (not (> (Components|Timeline|GetPlaybackPosition _openingventtimer) (- (Components|Timeline|GetTimelineLength _openingventtimer) 0.5)))
        (CallFunction|Close)))))

(event Custom|Close
  (Variables|Default|SetisRevealedByLight true)
  (Collision|SetCollisionResponsetoChannel (Variables|Default|GetObjectBodyToBeRevealed) "ECC_GameTraceChannel2" "ECR_Block")
  (if (< (Variables|Default|GetLightSources) 1)
    (CallFunction|Hide)))

(event EventBeginPlay
  (bind _openingventtimer (Variables|Default|GetOpeningVentTimer))
  (|CallParentFunction)
  (Components|Timeline|SetPlayRate _openingventtimer (/ (Components|Timeline|GetTimelineLength _openingventtimer) (Variables|Default|GetTimeSpeedToOpen))))

(event EventInteract
  (if (Utilities|Array|IsValidIndex (Collision|GetOverlappingActors (Variables|Default|GetOpeningDistanceCheck) "/Game/FirstPerson/Blueprints/BP_FirstPersonCharacter.BP_FirstPersonCharacter_C" :!class /Script/Engine.PrimitiveComponent))
    (CallFunction|Open)))

(event EventTick
  (params (DeltaSeconds :type Float%20%28single-precision%29))
  (Development|PrintString (Utilities|String|ToString(Integer) (Variables|Default|GetLightSources))))

(event EventHide
  (params (Component :type Static%20Mesh%20Component%20Object%20Reference) (SphereCollision :type Sphere%20Component%20Object%20Reference))
  (|CallParentFunction 0 0))

(fn ConstructionScript
  (|CallParentFunction))