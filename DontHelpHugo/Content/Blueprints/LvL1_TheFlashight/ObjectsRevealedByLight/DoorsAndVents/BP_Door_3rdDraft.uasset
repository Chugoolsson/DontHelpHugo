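; Swinging door revealed by light that players and enemies can pass through, with enemies opening it automatically on contact.
; Side A/B overlap counts set the swing direction, favoring the player, and a random-delay timer starts the hinge timeline only while light sources remain.
; The door reverses closed when its closing volume empties or, via Hide, when light runs out, unless the open timer is pending.
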(event OnComponentBeginOverlap(SideACollision)
  (params (OverlappedComponent :type Primitive%20Component%20Object%20Reference) (OtherActor :type Actor%20Object%20Reference) (OtherComp :type Primitive%20Component%20Object%20Reference) (OtherBodyIndex :type Integer) (bFromSweep :type Boolean) (SweepResult :type Hit%20Result%20Structure%20%28by%20ref%29))
  (bind _returnvalue (Utilities|GetClass OtherActor))
  (bind _returnvalue_2 (== _returnvalue "/Game/Blueprints/Test/AI/BP_BaseEnemy.BP_BaseEnemy_C"))
  (if (or (== _returnvalue "/Game/FirstPerson/Blueprints/BP_FirstPersonCharacter.BP_FirstPersonCharacter_C") _returnvalue_2)
    (Math|Integer|IncrementInt (Variables|DoorVariables|GetSideA)
      (:%20%20
        (if _returnvalue_2
          (CallFunction|Interact))))))

(event OnComponentEndOverlap(SideACollision)
  (params (OverlappedComponent :type Primitive%20Component%20Object%20Reference) (OtherActor :type Actor%20Object%20Reference) (OtherComp :type Primitive%20Component%20Object%20Reference) (OtherBodyIndex :type Integer))
  (bind _returnvalue (Utilities|GetClass OtherActor))
  (if (or (== _returnvalue "/Game/FirstPerson/Blueprints/BP_FirstPersonCharacter.BP_FirstPersonCharacter_C") (== _returnvalue "/Game/Blueprints/Test/AI/BP_BaseEnemy.BP_BaseEnemy_C"))
    (Math|Integer|DecrementInt (Variables|DoorVariables|GetSideA)
      (:%20%20
        (if (and (not (Utilities|IsPlayerorEnemyInsideDoorClosingCollision)) (Variables|DoorVariables|GetisOpen))
          (CallFunction|CloseDoor))))))

(event OnComponentEndOverlap(DoorClosingCollision2)
  (params (OverlappedComponent :type Primitive%20Component%20Object%20Reference) (OtherActor :type Actor%20Object%20Reference) (OtherComp :type Primitive%20Component%20Object%20Reference) (OtherBodyIndex :type Integer))
  (bind _doorclosingcollision2 (Variables|Default|GetDoorClosingCollision2))
  (if (Math|Boolean|ANDBoolean (Variables|Default|GetIsOpen) (== (Utilities|GetClass OtherActor) "/Game/Blueprints/Test/AI/BP_BaseEnemy.BP_BaseEnemy_C") (not (Utilities|Array|IsValidIndex (Collision|GetOverlappingActors _doorclosingcollision2 "/Game/FirstPerson/Blueprints/BP_FirstPersonCharacter.BP_FirstPersonCharacter_C" :!class /Script/Engine.PrimitiveComponent))) (not (Utilities|Array|IsValidIndex (Collision|GetOverlappingActors _doorclosingcollision2 "/Game/Blueprints/Test/AI/BP_BaseEnemy.BP_BaseEnemy_C" :!class /Script/Engine.PrimitiveComponent))) (not (Utilities|Time|IsTimerActivebyHandle (Variables|DoorVariables|GetWaitingToRotateDoorTimeHandle))))
    (for _array_element (Variables|Default|GetStuckedObjects)
      (Class|BISomethingIsStuckonYou|RemoveStuckedObject(Message) _array_element))
    (CallFunction|CloseDoor)))

(event OnComponentBeginOverlap(DoorClosingCollision2)
  (params (OverlappedComponent :type Primitive%20Component%20Object%20Reference) (OtherActor :type Actor%20Object%20Reference) (OtherComp :type Primitive%20Component%20Object%20Reference) (OtherBodyIndex :type Integer) (bFromSweep :type Boolean) (SweepResult :type Hit%20Result%20Structure%20%28by%20ref%29))
  (if (and (== (Utilities|GetClass OtherActor) "/Game/Blueprints/Test/AI/BP_BaseEnemy.BP_BaseEnemy_C") (not (Variables|DoorVariables|GetisOpen)))
    _))

(event OnComponentEndOverlap(SideBCollision)
  (params (OverlappedComponent :type Primitive%20Component%20Object%20Reference) (OtherActor :type Actor%20Object%20Reference) (OtherComp :type Primitive%20Component%20Object%20Reference) (OtherBodyIndex :type Integer))
  (bind _returnvalue (Utilities|GetClass OtherActor))
  (if (or (== _returnvalue "/Game/FirstPerson/Blueprints/BP_FirstPersonCharacter.BP_FirstPersonCharacter_C") (== _returnvalue "/Game/Blueprints/Test/AI/BP_BaseEnemy.BP_BaseEnemy_C"))
    (Math|Integer|DecrementInt (Variables|DoorVariables|GetSideB)
      (:%20%20
        (if (and (not (Utilities|IsPlayerorEnemyInsideDoorClosingCollision)) (Variables|DoorVariables|GetisOpen))
          (CallFunction|CloseDoor))))))

(event OnComponentBeginOverlap(SideBCollision)
  (params (OverlappedComponent :type Primitive%20Component%20Object%20Reference) (OtherActor :type Actor%20Object%20Reference) (OtherComp :type Primitive%20Component%20Object%20Reference) (OtherBodyIndex :type Integer) (bFromSweep :type Boolean) (SweepResult :type Hit%20Result%20Structure%20%28by%20ref%29))
  (bind _returnvalue (Utilities|GetClass OtherActor))
  (bind _returnvalue_2 (== _returnvalue "/Game/Blueprints/Test/AI/BP_BaseEnemy.BP_BaseEnemy_C"))
  (if (or (== _returnvalue "/Game/FirstPerson/Blueprints/BP_FirstPersonCharacter.BP_FirstPersonCharacter_C") _returnvalue_2)
    (Math|Integer|IncrementInt (Variables|DoorVariables|GetSideB)
      (:%20%20
        (if _returnvalue_2
          (CallFunction|Interact))))))

(event Custom|RotatingDoor
  (if (> (Variables|Default|GetLightSources) 0)
    (CallFunction|PrioritizePlayerifRelevant)
    (for _array_element (Variables|Default|GetStuckedObjects)
      (Class|BISomethingIsStuckonYou|RemoveStuckedObject(Message) _array_element))
    (bind _alpha (Timeline|RotateDoor Play)
      (:Update
        (Transformation|SetRelativeRotation (Variables|Default|GetDoorRotationPoint) (Math|Rotator|Lerp(Rotator) (Variables|DoorVariables|GetCurrentRotation) (Variables|DoorVariables|GetRotateDestination) _alpha) false false))
      (:Finished
        (if (<= _alpha 0.5)
          (CallFunction|SetDoorasNotOpen)
          (elif (not (Utilities|IsPlayerorEnemyInsideDoorClosingCollision))
            (CallFunction|CloseDoor)))))
    (else
      (CallFunction|SetDoorasNotOpen))))

(event Custom|CloseDoor
  (if (and (<= (Variables|Default|GetPlayerInSafePassage) 0) (not (Utilities|Time|IsTimerActivebyHandle (Variables|DoorVariables|GetWaitingToRotateDoorTimeHandle))))
    (bind _alpha (Timeline|RotateDoor Reverse)
      (:Update
        (Transformation|SetRelativeRotation (Variables|Default|GetDoorRotationPoint) (Math|Rotator|Lerp(Rotator) (Variables|DoorVariables|GetCurrentRotation) (Variables|DoorVariables|GetRotateDestination) _alpha) false false))
      (:Finished
        (if (<= _alpha 0.5)
          (CallFunction|SetDoorasNotOpen)
          (elif (not (Utilities|IsPlayerorEnemyInsideDoorClosingCollision))
            (CallFunction|CloseDoor)))))))

(event EventBeginPlay
  (bind _rotatedoor (Variables|Default|GetRotateDoor))
  (|CallParentFunction)
  (CallFunction|SetDoorRotationPointasParent)
  (Components|Timeline|SetPlayRate _rotatedoor (/ (Components|Timeline|GetTimelineLength _rotatedoor) (Variables|DoorVariables|GetDoorRotationTime))))

(event EventInteract
  (if (not (Variables|DoorVariables|GetisOpen))
    (Variables|DoorVariables|SetisOpen true)
    (Collision|SetCollisionResponsetoChannel (Variables|Default|GetObjectBodyToBeRevealed) "ECC_GameTraceChannel2" "ECR_Ignore")
    (Variables|DoorVariables|SetCurrentRotation (Variables|/Script/Engine.SceneComponent|GetRelativeRotation (Variables|Default|GetDoorRotationPoint)))
    (if (== (Variables|DoorVariables|GetSideA) 0)
      (Variables|DoorVariables|SetRotateDestination (Math|Rotator|MakeRotator 0.0 0.0 (+ (.yaw (Variables|DoorVariables|GetCurrentRotation)) -9e+01)))
      (else
        (Variables|DoorVariables|SetRotateDestination (Math|Rotator|MakeRotator 0.0 0.0 (+ (.yaw (Variables|DoorVariables|GetCurrentRotation)) 9e+01)))))
    (bind _returnvalue (Utilities|Time|SetTimerbyEvent (delegate Custom|RotatingDoor) (Math|Random|RandomFloatinRange (Variables|DoorVariables|GetMinimumTimeToStartRotate) (Variables|DoorVariables|GetMaximumTimeToStartRotate))))
    (Variables|DoorVariables|SetWaitingToRotateDoorTimeHandle _returnvalue)))

(event EventLeftSafePassagewithZeroLightSOurcesonObject
  (bind _doorrotationpoint (Variables|Default|GetDoorRotationPoint))
  (bind _relativerotation (Variables|/Script/Engine.SceneComponent|GetRelativeRotation _doorrotationpoint))
  (if (or (and (== (Variables|DoorVariables|GetSideB) 1) (<= (.yaw _relativerotation) -8e+01)) (and (>= (.yaw _relativerotation) 8e+01) (== (Variables|DoorVariables|GetSideA) 1)))
    (CallFunction|Hide)))

(event EventHide
  (params (Component :type Static%20Mesh%20Component%20Object%20Reference) (SphereCollision :type Sphere%20Component%20Object%20Reference))
  (if (and (Variables|DoorVariables|GetisOpen) (not (Utilities|Time|IsTimerActivebyHandle (Variables|DoorVariables|GetWaitingToRotateDoorTimeHandle))))
    (bind _output_get (CallFunction|SubtractLightSource))
    (if (<= _output_get 0)
      (CallFunction|CloseDoor))
    (else
      (|CallParentFunction 0 0))))

(fn ConstructionScript
  (|CallParentFunction))

(fn SetDoorRotationPointasParent
  (bind _doorrotationpoint (Variables|Default|GetDoorRotationPoint))
  (bind _objectbodytoberevealed (Variables|Default|GetObjectBodyToBeRevealed))
  (bind _staticmesh (Variables|/Script/Engine.StaticMeshComponent|GetStaticMesh _objectbodytoberevealed))
  (bind _returnvalue (StaticMesh|GetBoundingBox _staticmesh))
  (bind (_min _max) (Utilities|Struct|BreakBox _returnvalue))
  (Transformation|SetWorldLocation _doorrotationpoint (- (Transformation|GetWorldLocation _doorrotationpoint) (* (Math|Vector|GetRightVector _doorrotationpoint) (/ (- (.y _max) (.y _min)) 2.0))) false false)
  (Transformation|AttachComponentToComponent (Variables|Default|GetObjectBodyToBeRevealed) (Variables|Default|GetDoorRotationPoint) "None" "KeepWorld" "KeepWorld" "KeepWorld" true))

(fn SetDoorasNotOpen
  (Variables|Default|SetIsOpen false)
  (Collision|SetCollisionResponsetoChannel (Variables|Default|GetObjectBodyToBeRevealed) "ECC_GameTraceChannel2" "ECR_Block")
  (if (<= (Variables|Default|GetLightSources) 0)
    (CallFunction|Hide)))

(fn PrioritizePlayerifRelevant
  (if (or (Utilities|Array|IsValidIndex (Collision|GetOverlappingActors (Variables|Default|GetSideACollision) "/Game/FirstPerson/Blueprints/BP_FirstPersonCharacter.BP_FirstPersonCharacter_C" :!class /Script/Engine.PrimitiveComponent)) (Utilities|Array|IsValidIndex (Collision|GetOverlappingActors (Variables|Default|GetSideBCollision) "/Game/FirstPerson/Blueprints/BP_FirstPersonCharacter.BP_FirstPersonCharacter_C" :!class /Script/Engine.PrimitiveComponent)))
    (if (Utilities|Array|IsValidIndex (Collision|GetOverlappingActors (Variables|Default|GetSideACollision) "/Game/FirstPerson/Blueprints/BP_FirstPersonCharacter.BP_FirstPersonCharacter_C" :!class /Script/Engine.PrimitiveComponent))
      (Variables|DoorVariables|SetRotateDestination (Math|Rotator|MakeRotator 0.0 0.0 (+ (.yaw (Variables|DoorVariables|GetCurrentRotation)) 9e+01)))
      (else
        (Variables|DoorVariables|SetRotateDestination (Math|Rotator|MakeRotator 0.0 0.0 (+ (.yaw (Variables|DoorVariables|GetCurrentRotation)) -9e+01)))))))