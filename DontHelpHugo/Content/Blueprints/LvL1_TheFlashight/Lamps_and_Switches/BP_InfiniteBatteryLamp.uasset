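; Interactable lamp that toggles on and off and reveals hidden content within its light.
; BeginPlay applies the configured On state after a short delay, and Interact switches it through TurnOn and TurnOff.
; Both toggle the SpotLight and the LightReveal volume's visibility and query collision together.
; Overlapping actors get RevealMessage or HideMessage through their CBP_Reveal component, falling back to the BI_Reveal interface.
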(event OnComponentBeginOverlap(LightReveal)
  (params (OverlappedComponent :type Primitive%20Component%20Object%20Reference) (OtherActor :type Actor%20Object%20Reference) (OtherComp :type Primitive%20Component%20Object%20Reference) (OtherBodyIndex :type Integer) (bFromSweep :type Boolean) (SweepResult :type Hit%20Result%20Structure%20%28by%20ref%29))
  (bind _returnvalue (Actor|GetComponentbyClass OtherActor "/Game/Blueprints/LvL1_TheFlashight/Actor_Components/CBP_Reveal.CBP_Reveal_C"))
  ;[1 0.31 0.8345] Reveal and hide styff within the light
  (Utilities|IsValid _returnvalue
    (:Is%20Valid
      (Class|BIReveal|Reveal(Message) _returnvalue))
    (:Is%20Not%20Valid
      (if (Utilities|DoesObjectImplementInterface OtherActor "/Game/Blueprints/LvL1_TheFlashight/Interfaces/BI_Reveal.BI_Reveal_C")
        (Class|BIReveal|Reveal(Message) OtherActor)))))

(event OnComponentEndOverlap(LightReveal)
  (params (OverlappedComponent :type Primitive%20Component%20Object%20Reference) (OtherActor :type Actor%20Object%20Reference) (OtherComp :type Primitive%20Component%20Object%20Reference) (OtherBodyIndex :type Integer))
  (bind _returnvalue (Actor|GetComponentbyClass OtherActor "/Game/Blueprints/LvL1_TheFlashight/Actor_Components/CBP_Reveal.CBP_Reveal_C"))
  ;[1 0.31 0.8345] Reveal and hide styff within the light
  (Utilities|IsValid _returnvalue
    (:Is%20Valid
      (Class|BIReveal|Hide(Message) _returnvalue))
    (:Is%20Not%20Valid
      (if (Utilities|DoesObjectImplementInterface OtherActor "/Game/Blueprints/LvL1_TheFlashight/Interfaces/BI_Reveal.BI_Reveal_C")
        (Class|BIReveal|Hide(Message) OtherActor)))))

(event EventInteract
  (if (Variables|Default|GetOn)
    (CallFunction|TurnOff)
    (else
      (CallFunction|Turnon))))

(event EventBeginPlay
  (bind _spotlight (Variables|Default|GetSpotLight))
  (bind _lightreveal (Variables|Default|GetLightReveal))
  (bind _lightreveal_2 (Variables|Default|GetLightReveal))
  (bind _lightreveal_3 (Variables|Default|GetLightReveal))
  ;[0.3127 1 0.8255] Seting up and make it so to choose if it should start on or off
  (Collision|SetCollisionEnabled _lightreveal_2 "NoCollision")
  (Rendering|SetVisibility _lightreveal_2 false false)
  (Utilities|FlowControl|Delay 0.2)
  (if (Variables|Default|GetOn)
    (Rendering|SetVisibility _spotlight true false)
    (Collision|SetCollisionEnabled _lightreveal "QueryOnly")
    (Rendering|SetVisibility _lightreveal true false)
    (else
      (Rendering|SetVisibility _spotlight false false)
      (Collision|SetCollisionEnabled _lightreveal_3 "NoCollision")
      (Rendering|SetVisibility _lightreveal_3 false false))))

(fn ConstructionScript)

(fn TurnOff
  (bind _lightreveal (Variables|Default|GetLightReveal))
  (Rendering|SetVisibility (Variables|Default|GetSpotLight) false false)
  (Variables|Default|SetOn false)
  (Collision|SetCollisionEnabled _lightreveal "NoCollision")
  (Rendering|SetVisibility _lightreveal false false))

(fn Turnon
  (bind _lightreveal (Variables|Default|GetLightReveal))
  (Rendering|SetVisibility (Variables|Default|GetSpotLight) true false)
  (Variables|Default|SetOn true)
  (Collision|SetCollisionEnabled _lightreveal "QueryOnly")
  (Rendering|SetVisibility _lightreveal true false))