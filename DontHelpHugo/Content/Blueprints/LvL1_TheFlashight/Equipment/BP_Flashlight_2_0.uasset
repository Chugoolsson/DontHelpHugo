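; Battery-powered flashlight equipment that reveals objects inside its light and can fire bullets at a battery cost.
; RevealCollision overlaps show or hide targets through CBP_Reveal, falling back to the older BI_Reveal interface.
; A self-restarting BatteryTimeline acts as a variable-rate timer for draining, charging or randomized flickering, according to the battery state enum.
; Light and reveal collision toggle together, and battery changes update the UI widget.
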(event OnComponentBeginOverlap(RevealCollision)
  (params (OverlappedComponent :type Primitive%20Component%20Object%20Reference) (OtherActor :type Actor%20Object%20Reference) (OtherComp :type Primitive%20Component%20Object%20Reference) (OtherBodyIndex :type Integer) (bFromSweep :type Boolean) (SweepResult :type Hit%20Result%20Structure%20%28by%20ref%29))
  (bind _returnvalue (Actor|GetComponentbyClass OtherActor "/Game/Blueprints/LvL1_TheFlashight/Actor_Components/CBP_Reveal.CBP_Reveal_C"))
  ;[1 0.7043 0.008784] Calling the reveal inteface when an object enters the light and leaving. Get component by class is the new way and the "does implement interface" is for the old way of doing this.
  (Utilities|IsValid _returnvalue
    (:Is%20Valid
      (Class|BIReveal|Reveal(Message) _returnvalue))
    (:Is%20Not%20Valid
      (if (Utilities|DoesObjectImplementInterface OtherActor "/Game/Blueprints/LvL1_TheFlashight/Interfaces/BI_Reveal.BI_Reveal_C")
        (Class|BIReveal|Reveal(Message) OtherActor)))))

(event OnComponentEndOverlap(RevealCollision)
  (params (OverlappedComponent :type Primitive%20Component%20Object%20Reference) (OtherActor :type Actor%20Object%20Reference) (OtherComp :type Primitive%20Component%20Object%20Reference) (OtherBodyIndex :type Integer))
  (bind _returnvalue (Actor|GetComponentbyClass OtherActor "/Game/Blueprints/LvL1_TheFlashight/Actor_Components/CBP_Reveal.CBP_Reveal_C"))
  ;[1 0.7043 0.008784] Calling the reveal inteface when an object enters the light and leaving. Get component by class is the new way and the "does implement interface" is for the old way of doing this.
  (Utilities|IsValid _returnvalue
    (:Is%20Valid
      (Class|BIReveal|Hide(Message) _returnvalue))
    (:Is%20Not%20Valid
      (if (Utilities|DoesObjectImplementInterface OtherActor "/Game/Blueprints/LvL1_TheFlashight/Interfaces/BI_Reveal.BI_Reveal_C")
        (Class|BIReveal|Hide(Message) OtherActor)))))

(event Custom|Event%20OutOfBattery
  (bind _batterytimeline (Variables|Default|GetBatteryTimeline))
  ;[0.446 0.593 1] Loosing and charging the battery based on state
  (|SetBy-RefVar (Variables|Default|GetEnum) "NewEnumerator2")
  (Components|Timeline|SetPlayRate _batterytimeline (/ (Components|Timeline|GetTimelineLength _batterytimeline) (Math|Random|RandomFloatinRange (Variables|Default|GetMinimumFlickerDuration) (Variables|Default|GetMaximumFlickerDuration))))
  (Variables|Default|SetFlickerCount 0)
  (CallFunction|BatteryCheck))

(event Custom|BatteryCheck
  (bind _batterytimeline (Variables|Default|GetBatteryTimeline))
  (bind _batterytimeline_2 (Variables|Default|GetBatteryTimeline))
  ;[0.446 0.593 1] Loosing and charging the battery based on state
  (Timeline|BatteryTimeline PlayFromStart
    (:Finished
      (if (Variables|Default|GetpickedUp)
        (switch Utilities|FlowControl|Switch|SwitchonEnum_FlashLight (Variables|Default|GetEnum)
          (:NewEnumerator1
            (Variables|Default|SetCurrentBattery (Math|Float|Clamp(Float) (- (Variables|Default|GetCurrentBattery) (Variables|Default|GetReduceBattery)) 0.0 (Variables|Default|GetMaxBattery)))
            (Class|BIUpdateUI|UpdateUI(Message) (Variables|Default|GetWidgetUI_Ref) (/ (Variables|Default|GetCurrentBattery) (Variables|Default|GetMaxBattery)))
            (if (<= (Variables|Default|GetCurrentBattery) 0.0)
              (CallFunction|EventOutOfBattery)
              (else
                (CallFunction|BatteryCheck))))
          (:NewEnumerator0
            (Variables|Default|SetCurrentBattery (Math|Float|Clamp(Float) (+ (Variables|Default|GetCurrentBattery) (Variables|Default|GetAddBattery)) 0.0 (Variables|Default|GetMaxBattery)))
            (Class|BIUpdateUI|UpdateUI(Message) (Variables|Default|GetWidgetUI_Ref) (/ (Variables|Default|GetCurrentBattery) (Variables|Default|GetMaxBattery)))
            (if (>= (Variables|Default|GetCurrentBattery) (Variables|Default|GetMaxBattery))
              (|SetBy-RefVar (Variables|Default|GetEnum) "NewEnumerator1")
              (CallFunction|TurnonLightCollision)
              (Components|Timeline|SetPlayRate _batterytimeline_2 (/ (Components|Timeline|GetTimelineLength _batterytimeline_2) (Variables|Default|GetLoosingBatterTimeInterval)))
              (CallFunction|BatteryCheck)
              (else
                (CallFunction|BatteryCheck))))
          (:NewEnumerator2
            (Components|Timeline|SetPlayRate _batterytimeline (/ (Components|Timeline|GetTimelineLength _batterytimeline) (Math|Random|RandomFloatinRange (Variables|Default|GetMinimumFlickerDuration) (Variables|Default|GetMaximumFlickerDuration))))
            (Utilities|FlowControl|FlipFlop
              (:A
                (if (not (>= (Variables|Default|GetFlickerCount) (Variables|Default|GetFlickerAmountLimit)))
                  (CallFunction|TurnOffLightCollision)
                  (CallFunction|BatteryCheck)))
              (:B
                (bind _result (Math|Integer|IncrementInt (Variables|Default|GetFlickerCount))
                  (:%20%20
                    (if (not (>= _result (Variables|Default|GetFlickerAmountLimit)))
                      (CallFunction|TurnonLightCollision)
                      (CallFunction|BatteryCheck))))))))))))

(event Event1stEquipmentAbility
  ;[0.7387 1 0.02329] Shooting away the "Flashlight bullet"" if their is battery to use
  (switch Utilities|FlowControl|Switch|SwitchonEnum_FlashLight (Variables|Default|GetEnum)
    (:NewEnumerator1
      (if (>= (Variables|Default|GetCurrentBattery) (Variables|Default|GetBatteryReducedByBullet))
        (CallFunction|ShootBullet)
        (if (<= (Variables|Default|GetCurrentBattery) 0.0)
          (CallFunction|EventOutOfBattery))))))

(event Event3rdEquipmentAbility
  (bind _batterytimeline (Variables|Default|GetBatteryTimeline))
  ;[0.3038 1 0] Starting to charge the battery and go into "charging" state
  (|SetBy-RefVar (Variables|Default|GetEnum) "NewEnumerator0")
  (CallFunction|BatteryCheck)
  (Components|Timeline|SetPlayRate _batterytimeline (/ (Components|Timeline|GetTimelineLength _batterytimeline) (Variables|Default|GetChargingBatteryTimeInterval)))
  (CallFunction|TurnOffLightCollision)
  (Class|BIUpdateUI|UIEquipmentAbility3(Message) (Variables|Default|GetWidgetUI_Ref)))

(event EventBeginPlay
  (bind _maxbattery (Variables|Default|GetMaxBattery))
  (|CallParentFunction)
  (bind _output_get (Variables|Default|SetCurrentBattery _maxbattery))
  (Class|BIUpdateUI|UpdateUI(Message) (Variables|Default|GetWidgetUI_Ref) (/ _output_get _maxbattery)))

(event EventPickedUp
  (|CallParentFunction)
  (CallFunction|BatteryCheck))

(event Event4thEquipmentAbility
  (bind _batterytimeline (Variables|Default|GetBatteryTimeline))
  (bind _enum (Variables|Default|GetEnum))
  ;[0.4209 1 0.7196] Stop charging and switshing back to loosing battery
  (if (>= 1.0 (Variables|Default|GetCurrentBattery))
    (|SetBy-RefVar _enum "NewEnumerator2")
    (else
      (|SetBy-RefVar _enum "NewEnumerator1")
      (if (not (<= (Variables|Default|GetCurrentBattery) 0.0))
        (CallFunction|TurnonLightCollision)
        (Components|Timeline|SetPlayRate _batterytimeline (/ (Components|Timeline|GetTimelineLength _batterytimeline) (Variables|Default|GetLoosingBatterTimeInterval)))
        (CallFunction|BatteryCheck)))))

(fn ConstructionScript
  (|CallParentFunction))

(fn SetUpWidgets)

(fn ShootBullet
  (bind _bulletspawn (Variables|Default|GetBulletSpawn))
  (Game|SpawnActorfromClass "/Game/Blueprints/LvL1_TheFlashight/Equipment/BP_FlashlightBullet.BP_FlashlightBullet_C" (Math|Transform|MakeTransform (Transformation|GetWorldLocation _bulletspawn) (Transformation|GetWorldRotation _bulletspawn)) "Undefined" "MultiplyWithRoot" 0 0)
  (bind _output_get (Variables|Default|SetCurrentBattery (- (Variables|Default|GetCurrentBattery) (Variables|Default|GetBatteryReducedByBullet))))
  (Class|BIUpdateUI|UpdateUI(Message) (Variables|Default|GetWidgetUI_Ref) (/ _output_get (Variables|Default|GetMaxBattery)))
  (CallFunction|BatteryCheck))

(fn TurnOffLightCollision
  (Collision|SetCollisionEnabled (Variables|Default|GetRevealCollision) "NoCollision")
  (Rendering|SetVisibility (Variables|Default|GetSpotLight) false false)
  (Rendering|SetVisibility (Variables|Default|GetRevealCollision) false false))

(fn TurnonLightCollision
  (Collision|SetCollisionEnabled (Variables|Default|GetRevealCollision) "QueryOnly")
  (Rendering|SetVisibility (Variables|Default|GetSpotLight) true false)
  (Rendering|SetVisibility (Variables|Default|GetRevealCollision) true false))