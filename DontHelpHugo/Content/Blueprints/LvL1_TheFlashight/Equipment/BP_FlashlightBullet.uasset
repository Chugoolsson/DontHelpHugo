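; Glowing flashlight projectile that lights its surroundings and reveals hidden actors within its trigger sphere, via CBP_Reveal or the BI_Reveal interface.
; After a timed delay, a timeline animates glow, light and reveal size, then removes those components and enables physics.
; It briefly enables bouncing when hitting enemies, the player or other bullets.
; It notifies other hit actors that it is stuck, and RemoveStuckedObject frees it with physics.
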(event OnComponentHit(Object)
  (params (HitComponent :type Primitive%20Component%20Object%20Reference) (OtherActor :type Actor%20Object%20Reference) (OtherComp :type Primitive%20Component%20Object%20Reference) (NormalImpulse :type Vector :default "0, 0, 0") (Hit :type Hit%20Result%20Structure%20%28by%20ref%29))
  (bind _returnvalue (Utilities|GetClass OtherActor))
  ;[0.6291 0.4112 1] Bouncing way in case hitting certain actors
  (if (Math|Boolean|ORBoolean (== _returnvalue "/Game/Blueprints/Test/AI/BP_BaseEnemy.BP_BaseEnemy_C") (== _returnvalue "BP_FlashlightBullet_C") (== _returnvalue "/Game/FirstPerson/Blueprints/BP_FirstPersonCharacter.BP_FirstPersonCharacter_C"))
    (Variables|/Script/Engine.ProjectileMovementComponent|SetbShouldBounce (Variables|Default|GetProjectileMovement) true)
    (Utilities|FlowControl|Delay 0.05)
    (Variables|/Script/Engine.ProjectileMovementComponent|SetbShouldBounce (Variables|Default|GetProjectileMovement) false)
    (else
      (Class|BISomethingIsStuckonYou|ObjectGotStucked(Message) OtherActor self))))

(event OnComponentBeginOverlap(LightTrigger)
  (params (OverlappedComponent :type Primitive%20Component%20Object%20Reference) (OtherActor :type Actor%20Object%20Reference) (OtherComp :type Primitive%20Component%20Object%20Reference) (OtherBodyIndex :type Integer) (bFromSweep :type Boolean) (SweepResult :type Hit%20Result%20Structure%20%28by%20ref%29))
  (bind _returnvalue (Actor|GetComponentbyClass OtherActor "/Game/Blueprints/LvL1_TheFlashight/Actor_Components/CBP_Reveal.CBP_Reveal_C"))
  (Utilities|IsValid _returnvalue
    (:Is%20Valid
      (Class|BIReveal|Reveal(Message) _returnvalue))
    (:Is%20Not%20Valid
      (if (Utilities|DoesObjectImplementInterface OtherActor "/Game/Blueprints/LvL1_TheFlashight/Interfaces/BI_Reveal.BI_Reveal_C")
        (Class|BIReveal|Reveal(Message) OtherActor)))))

(event OnComponentEndOverlap(LightTrigger)
  (params (OverlappedComponent :type Primitive%20Component%20Object%20Reference) (OtherActor :type Actor%20Object%20Reference) (OtherComp :type Primitive%20Component%20Object%20Reference) (OtherBodyIndex :type Integer))
  (bind _returnvalue (Actor|GetComponentbyClass OtherActor "/Game/Blueprints/LvL1_TheFlashight/Actor_Components/CBP_Reveal.CBP_Reveal_C"))
  (Utilities|IsValid _returnvalue
    (:Is%20Valid
      (Class|BIReveal|Hide(Message) _returnvalue))
    (:Is%20Not%20Valid
      (if (Utilities|DoesObjectImplementInterface OtherActor "/Game/Blueprints/LvL1_TheFlashight/Interfaces/BI_Reveal.BI_Reveal_C")
        (Class|BIReveal|Hide(Message) OtherActor)))))

(event Custom|TimeLineToCountDown
  (Timeline|TimelineToStartLifeSpan Play
    (:Finished
      (CallFunction|LifeSpan))))

(event Custom|LifeSpan
  ;[1 0.4754 0.1624] Making it fade and "stop" working slowly but steady
  (bind (_direction _emissiceglowvalue _lightintensity _lightcollisionsize _set__light__revealer_size) (Timeline|LifeSpanCountDown Play)
    (:Update
      (Rendering|Material|SetScalarParameterValue (Variables|Default|GetEmissiveValueMaterial) "Glow" _emissiceglowvalue :!class /Script/Engine.MaterialInstanceDynamic)
      (Rendering|Components|Light|SetIntensity (Variables|Default|GetPointLight) _lightintensity)
      (Components|Sphere|SetSphereRadius (Variables|Default|GetLightTrigger) _lightcollisionsize true)
      (Transformation|SetRelativeScale3D (Variables|Default|GetLightRevealer) _set__light__revealer_size))
    (:Finished
      (CallFunction|Death))))

(event Custom|Death
  (Components|DestroyComponent (Variables|Default|GetPointLight))
  (Components|DestroyComponent (Variables|Default|GetLightTrigger))
  (Components|DestroyComponent (Variables|Default|GetLightRevealer))
  (Physics|SetSimulatePhysics (Variables|Default|GetObject) true))

(event EventRemoveStuckedObject
  ;[0.1823 0.3985 1] When a door is opened for example and the bullet is stuck on it
  (Physics|SetSimulatePhysics (Variables|Default|GetObject) true))

(event EventBeginPlay
  (CallFunction|TimeLinetoCountDown)
  (CallFunction|CreateDynamicMaterial)
  (Components|Sphere|SetSphereRadius (Variables|Default|GetLightTrigger) 25.0 true))

(fn ConstructionScript)

(fn CreateDynamicMaterial
  (bind _returnvalue (Rendering|Material|CreateDynamicMaterialInstance "/Game/Materials/Material/Colors/MI_EmissiveWhite.MI_EmissiveWhite" "Glow" "None" :!class /Script/Engine.KismetMaterialLibrary))
  (bind _output_get (Variables|Default|SetEmissiveValueMaterial _returnvalue))
  (Rendering|Material|SetMaterial (Variables|Default|GetObject) 0 _output_get)
  (Rendering|Material|SetScalarParameterValue _output_get "Glow" 5.0 :!class /Script/Engine.MaterialInstanceDynamic))