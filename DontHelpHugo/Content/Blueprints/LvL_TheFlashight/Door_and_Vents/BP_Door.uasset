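; Interactable door Blueprint that swings its mesh 90 degrees in yaw around a side hinge when Interact fires.
; BeginPlay moves an ANCHOR component to the door's edge, offset by half the mesh's bounding-box width.
; A timeline scaled by OpeningDoorTime drives RInterpTo on the anchor, then copies its rotation to the door and repositions it from that pivot.
; Spline-path nodes are disconnected and never run.
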(event EventBeginPlay
  (bind _object (Variables|Default|GetObject))
  (bind _staticmesh (Variables|/Script/Engine.StaticMeshComponent|GetStaticMesh _object))
  (bind _returnvalue (StaticMesh|GetBoundingBox _staticmesh))
  (bind (_min _max) (Utilities|Struct|BreakBox _returnvalue))
  (|CallParentFunction)
  (Transformation|SetWorldLocationAndRotation (Variables|Default|Get"ANCHOR") (- (Variables|/Script/Engine.SceneComponent|GetRelativeLocation _object) (* (Math|Vector|GetRightVector _object) (/ (- (.y _max) (.y _min)) 2.0))) "0, 0, 0" false false))

(event EventInteract
  (bind __anchor_ (Variables|Default|Get"ANCHOR"))
  (bind __anchor__2 (Variables|Default|Get"ANCHOR"))
  (bind _object (Variables|Default|GetObject))
  (bind _object_2 (Variables|Default|GetObject))
  (bind _object_3 (Variables|Default|GetObject))
  (bind _staticmesh (Variables|/Script/Engine.StaticMeshComponent|GetStaticMesh _object_3))
  (bind _relativelocation (Variables|/Script/Engine.SceneComponent|GetRelativeLocation _object_3))
  (bind _returnvalue (StaticMesh|GetBoundingBox _staticmesh))
  (bind (_min _max) (Utilities|Struct|BreakBox _returnvalue))
  (bind _returnvalue_2 (- (.y _max) (.y _min)))
  (bind _returnvalue_3 (/ _returnvalue_2 2.0))
  (Variables|Default|SetDoorStartPoint _relativelocation)
  (Variables|Default|SetDoorDestination (Utilities|Operators|Subtract _relativelocation (* (Math|Vector|GetForwardVector _object_3) _returnvalue_3) (* (Math|Vector|GetRightVector _object_3) _returnvalue_3)))
  (Variables|Default|SetCurrentRotation (Transformation|GetWorldRotation _object_2))
  (Variables|Default|SetRotateDegree (+ (.yaw (Transformation|GetWorldRotation _object_2)) 9e+01))
  (Components|Timeline|SetPlayRate (Variables|Default|GetRotatingDoor) (/ 1.0 (Variables|Default|GetOpeningDoorTime)))
  (bind _rotate (Timeline|RotatingDoor PlayFromStart)
    (:Update
      (Transformation|SetWorldRotation __anchor__2 (Math|Interpolation|RInterpTo (Variables|Default|GetCurrentRotation) (Math|Rotator|MakeRotator 0.0 0.0 (Variables|Default|GetRotateDegree)) _rotate 1e+01) false false)
      (Transformation|SetWorldRotation _object (Transformation|GetWorldRotation __anchor__2) false false)
      (Transformation|SetWorldLocation _object (+ (Transformation|GetWorldLocation __anchor_) (* (Math|Vector|GetRightVector __anchor_) _returnvalue_3)) false false))))

(fn ConstructionScript
  (|CallParentFunction))