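; Interactable swing door that rotates 90 degrees in a direction chosen by the player's side and closes automatically.
; On BeginPlay, it shifts ANCHOR by half the mesh width as a hinge and attaches the door.
; Interact ignores the Visibility channel, waits a random delay, then plays a duration-scaled timeline rotating ANCHOR.
; The timeline reverses once the player is outside the Sphere, restoring Visibility blocking when closed.
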(event OnComponentBeginOverlap(SideACollision)
  (params (OverlappedComponent :type Primitive%20Component%20Object%20Reference) (OtherActor :type Actor%20Object%20Reference) (OtherComp :type Primitive%20Component%20Object%20Reference) (OtherBodyIndex :type Integer) (bFromSweep :type Boolean) (SweepResult :type Hit%20Result%20Structure%20%28by%20ref%29))
  (if (== (Utilities|GetClass OtherActor) "/Game/FirstPerson/Blueprints/BP_FirstPersonCharacter.BP_FirstPersonCharacter_C")
    (Math|Integer|IncrementInt (Variables|Default|GetSideA))))

(event OnComponentEndOverlap(SideACollision)
  (params (OverlappedComponent :type Primitive%20Component%20Object%20Reference) (OtherActor :type Actor%20Object%20Reference) (OtherComp :type Primitive%20Component%20Object%20Reference) (OtherBodyIndex :type Integer))
  (if (== (Utilities|GetClass OtherActor) "/Game/FirstPerson/Blueprints/BP_FirstPersonCharacter.BP_FirstPersonCharacter_C")
    (bind _result (Math|Integer|DecrementInt (Variables|Default|GetSideA))
      (:%20%20
        (Variables|Default|SetSideA (Math|Integer|Clamp(Integer) _result 0 5))))))

(event OnComponentEndOverlap(Sphere)
  (params (OverlappedComponent :type Primitive%20Component%20Object%20Reference) (OtherActor :type Actor%20Object%20Reference) (OtherComp :type Primitive%20Component%20Object%20Reference) (OtherBodyIndex :type Integer))
  (if (and (Variables|Default|GetIsOpen) (== (Utilities|GetClass OtherActor) "/Game/FirstPerson/Blueprints/BP_FirstPersonCharacter.BP_FirstPersonCharacter_C"))
    (bind _alpha (Timeline|RotatingDoor Reverse)
      (:Update
        (Transformation|SetRelativeRotation (Variables|Default|GetANCHOR) (Math|Rotator|Lerp(Rotator) (Variables|Default|GetCurrentRotation) (Variables|Default|GetRotateDestination) _alpha) false false))
      (:Finished
        (if (<= _alpha 0.2)
          (Variables|Default|SetIsOpen false)
          (Collision|SetCollisionResponsetoChannel (Variables|Default|GetDoor) "ECC_Visibility" "ECR_Block")
          (elif (not (Utilities|Array|IsValidIndex (Collision|GetOverlappingActors (Variables|Default|GetSphere) "/Game/FirstPerson/Blueprints/BP_FirstPersonCharacter.BP_FirstPersonCharacter_C" :!class /Script/Engine.PrimitiveComponent)))
            (Timeline|RotatingDoor Reverse)))))))

(event EventBeginPlay
  (bind _rotatingdoor (Variables|Default|GetRotatingDoor))
  (CallFunction|SettingUpAnchorasParrent)
  (Components|Timeline|SetPlayRate _rotatingdoor (/ (Components|Timeline|GetTimelineLength _rotatingdoor) (Variables|Default|GetTimeToRotate))))

(event EventInteract
  (Variables|Default|SetIsOpen true)
  (Collision|SetCollisionResponsetoChannel (Variables|Default|GetDoor) "ECC_Visibility" "ECR_Ignore")
  (Variables|Default|SetCurrentRotation (Variables|/Script/Engine.SceneComponent|GetRelativeRotation (Variables|Default|GetANCHOR)))
  (if (== (Variables|Default|GetSideA) 0)
    (Variables|Default|SetRotateDestination (Math|Rotator|MakeRotator 0.0 0.0 (+ (.yaw (Variables|Default|GetCurrentRotation)) -9e+01)))
    (else
      (Variables|Default|SetRotateDestination (Math|Rotator|MakeRotator 0.0 0.0 (+ (.yaw (Variables|Default|GetCurrentRotation)) 9e+01)))))
  (Utilities|FlowControl|Delay (Math|Random|RandomFloatinRange (Variables|Default|GetMinimumTimeTostartRotate) (Variables|Default|GetMaximumTimeToStartRotate)))
  (bind _alpha (Timeline|RotatingDoor Play)
    (:Update
      (Transformation|SetRelativeRotation (Variables|Default|GetANCHOR) (Math|Rotator|Lerp(Rotator) (Variables|Default|GetCurrentRotation) (Variables|Default|GetRotateDestination) _alpha) false false))
    (:Finished
      (if (<= _alpha 0.2)
        (Variables|Default|SetIsOpen false)
        (Collision|SetCollisionResponsetoChannel (Variables|Default|GetDoor) "ECC_Visibility" "ECR_Block")
        (elif (not (Utilities|Array|IsValidIndex (Collision|GetOverlappingActors (Variables|Default|GetSphere) "/Game/FirstPerson/Blueprints/BP_FirstPersonCharacter.BP_FirstPersonCharacter_C" :!class /Script/Engine.PrimitiveComponent)))
          (Timeline|RotatingDoor Reverse))))))

(fn ConstructionScript)

(fn SettingUpAnchorasParrent
  (bind _door (Variables|Default|GetDoor))
  (bind _anchor (Variables|Default|GetANCHOR))
  (bind _staticmesh (Variables|/Script/Engine.StaticMeshComponent|GetStaticMesh _door))
  (bind _returnvalue (StaticMesh|GetBoundingBox _staticmesh))
  (bind (_min _max) (Utilities|Struct|BreakBox _returnvalue))
  (Transformation|SetWorldLocation _anchor (- (Transformation|GetWorldLocation _anchor) (* (Math|Vector|GetRightVector _anchor) (/ (- (.y _max) (.y _min)) 2.0))) false false)
  (Transformation|AttachComponentToComponent (Variables|Default|GetDoor) (Variables|Default|GetANCHOR) "None" "KeepWorld" "KeepWorld" "KeepWorld" true))