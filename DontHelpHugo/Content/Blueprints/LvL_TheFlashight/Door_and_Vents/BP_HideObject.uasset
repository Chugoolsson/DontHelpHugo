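; BP_HideObject is a wall-like object that becomes hidden and changes to a "Flashlight" collision profile while lit.
; Reveal and Hide events count active light sources, swapping the Body's material and collision profile.
; A SafePassage volume counts overlapping player characters, so Hide restores the solid wall only when no lights remain and the passage is empty.
; Leaving the passage only decrements the count and does not itself restore the wall.
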(event OnComponentBeginOverlap(SafePassage)
  (params (OverlappedComponent :type Primitive%20Component%20Object%20Reference) (OtherActor :type Actor%20Object%20Reference) (OtherComp :type Primitive%20Component%20Object%20Reference) (OtherBodyIndex :type Integer) (bFromSweep :type Boolean) (SweepResult :type Hit%20Result%20Structure%20%28by%20ref%29))
  ;[1 0.5168 0.1674] New way to hide an object inlight
  (if (== (Utilities|GetClass OtherActor) "/Game/FirstPerson/Blueprints/BP_FirstPersonCharacter.BP_FirstPersonCharacter_C")
    (Math|Integer|IncrementInt (Variables|Default|GetObjectsInSafePassage))))

(event OnComponentEndOverlap(SafePassage)
  (params (OverlappedComponent :type Primitive%20Component%20Object%20Reference) (OtherActor :type Actor%20Object%20Reference) (OtherComp :type Primitive%20Component%20Object%20Reference) (OtherBodyIndex :type Integer))
  ;[1 0.5168 0.1674] New way to hide an object inlight
  (if (== (Utilities|GetClass OtherActor) "/Game/FirstPerson/Blueprints/BP_FirstPersonCharacter.BP_FirstPersonCharacter_C")
    (Math|Integer|DecrementInt (Variables|Default|GetObjectsInSafePassage))))

(event EventReveal
  (params (Component :type Static%20Mesh%20Component%20Object%20Reference) (SphereCollision :type Sphere%20Component%20Object%20Reference))
  (bind _lightsource (Variables|Default|GetLightSource))
  ;[1 0.5168 0.1674] New way to hide an object inlight
  (Math|Integer|IncrementInt _lightsource
    (:%20%20
      (if (== _lightsource 1)
        (Rendering|Material|SetMaterial (Variables|Default|GetBody) 0 "/Game/Materials/Material/MI_Hide_NearestStaticMesh.MI_Hide_NearestStaticMesh")
        (CallFunction|TurnOffCollision)))))

(event EventHide
  (params (Component :type Static%20Mesh%20Component%20Object%20Reference) (SphereCollision :type Sphere%20Component%20Object%20Reference))
  ;[1 0.5168 0.1674] New way to hide an object inlight
  (bind _result (Math|Integer|DecrementInt (Variables|Default|GetLightSource))
    (:%20%20
      (Variables|Default|SetLightSource (Math|Integer|Clamp(Integer) _result 0 1000))
      (if (and (== (Variables|Default|GetLightSource) 0) (== (Variables|Default|GetObjectsInSafePassage) 0))
        (CallFunction|TurnonCollision)
        (Rendering|Material|SetMaterial (Variables|Default|GetBody) 0 "/Game/StarterContent/Materials/M_Basic_Wall.M_Basic_Wall")))))

(fn ConstructionScript)

(fn TurnOffCollision
  (Collision|SetCollisionProfileName (Variables|Default|GetBody) "Flashlight" true :!class /Script/Engine.PrimitiveComponent))

(fn TurnonCollision
  (Collision|SetCollisionProfileName (Variables|Default|GetBody) "PhysicsActor" true :!class /Script/Engine.PrimitiveComponent))