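; BP_LightSwitch is an interactable light switch that triggers its connected lamps one after another for a staged, thematic effect.
; Interact runs a delayed loop that walks the lamp array from last to first, sending InteractMessage to each lamp.
; When the counter passes the start of the array, it resets and reverses the array, so the next interaction runs in the opposite order.
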(event EventInteract
  (bind _lampsconnectetd (Variables|Default|GetLampsConnectetd))
  ;[0.712 0.3244 1] To be able to control the way lamps turs on for thematic effect
  (Utilities|FlowControl|Delay (Variables|Default|GetTimeToSwitchOn/Off) :!label _label)
  (Class|BIInteract|Interact(Message) (Utilities|Array|Get(acopy) (Variables|Default|GetLampsConnectetd) (- (Variables|Default|GetLampNextInLine) 1)))
  (Math|Integer|DecrementInt (Variables|Default|GetLampNextInLine)
    (:%20%20
      (if (== (Variables|Default|GetLampNextInLine) -1)
        (Variables|Default|SetLampNextInLine (Utilities|Array|Length _lampsconnectetd))
        (Utilities|Array|Reverse _lampsconnectetd)
        (else
          (goto _label))))))

(event EventBeginPlay
  ;[0.712 0.3244 1] To be able to control the way lamps turs on for thematic effect
  (Variables|Default|SetLampNextInLine (Utilities|Array|Length (Variables|Default|GetLampsConnectetd))))

(fn ConstructionScript
  (|CallParentFunction))